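; Test actor with two static mesh components that become simulated, colliding physics bodies at runtime.
; On BeginPlay, a sequence configures each mesh identically: physics simulation on, blocking all channels, query and physics collision, PhysicsBody object type.
; An unconnected leftover sets a collision profile by the name "BlackAllDynamic" and never runs.
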(event `self.ReceiveBeginPlay`
  (`|ExecutionSequence`
    (:`then_0`
      (`PrimitiveComponent.SetSimulatePhysics` (`self.StaticMesh`) true)
      (`PrimitiveComponent.SetCollisionResponseToAllChannels` (`self.StaticMesh`) "ECR_Block")
      (`PrimitiveComponent.SetCollisionEnabled` (`self.StaticMesh`) "QueryAndPhysics")
      (`PrimitiveComponent.SetCollisionObjectType` (`self.StaticMesh`) "ECC_PhysicsBody"))
    (:`then_1`
      (`PrimitiveComponent.SetSimulatePhysics` (`self.StaticMesh1`) true)
      (`PrimitiveComponent.SetCollisionResponseToAllChannels` (`self.StaticMesh1`) "ECR_Block")
      (`PrimitiveComponent.SetCollisionEnabled` (`self.StaticMesh1`) "QueryAndPhysics")
      (`PrimitiveComponent.SetCollisionObjectType` (`self.StaticMesh1`) "ECC_PhysicsBody"))))

(fn `UserConstructionScript`)