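; BP_Monitor is an interactable computer monitor that opens the WBP_Computer screen UI when clicked.
; Each Tick it polls the GlobalVariables game instance for whether it is the current HitResult and the left mouse is pressed.
; When both hold, it hides the crosshair, shows the cursor, creates the widget and switches input to UI only.
; No guard in this Blueprint prevents repeated widget creation while those conditions persist.
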(event `self.ReceiveTick`
  (params (DeltaSeconds :type "Float (single-precision)"))
  (bind _returnvalue (`GameplayStatics.GetPlayerController` 0))
  ;[1 1 1] Event Tick
  (`|ExecutionSequence`
    (:`then_0`
      (bind _asglobal_variables (cast `/Game/Workplace/Blueprints/GlobalVariables` (`GameplayStatics.GetGameInstance`)))
      (if (== self (`/Game/Workplace/Blueprints/GlobalVariables.HitResult` _asglobal_variables))
        (if (`/Game/Workplace/Blueprints/GlobalVariables.LeftMousePressed` _asglobal_variables)
          (set `/Game/Workplace/Blueprints/GlobalVariables.CrosshairVisible` false _asglobal_variables)
          (set `PlayerController.bShowMouseCursor` true _returnvalue)
          (bind _returnvalue_2 (`|CreateWidget` "/Game/Workplace/Menu/Blueprints/WBP_Computer.WBP_Computer_C"))
          (`UserWidget.AddToViewport` _returnvalue_2 1)
          (`WidgetBlueprintLibrary.SetInputMode_UIOnlyEx` _returnvalue _returnvalue_2))))))

(fn `UserConstructionScript`)