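; BP_Empty_Spool is a spool actor whose Plastic component appears only when the spool is flagged as Colored.
; BeginPlay clears the Colored flag, so Plastic starts hidden.
; Every Tick polls the flag, showing Plastic with the Material variable applied to its first slot when set, and hiding it otherwise.
; Nothing in this Blueprint sets Colored to true.
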(event `self.ReceiveBeginPlay`
  (set `self.Colored` false))

(event `self.ReceiveTick`
  (params (DeltaSeconds :type "Float (single-precision)"))
  (if (`self.Colored`)
    (`SceneComponent.SetVisibility` (`self.Plastic`) true false)
    (`PrimitiveComponent.SetMaterial` (`self.Plastic`) 0 (`self.Material`))
    (else
      (`SceneComponent.SetVisibility` (`self.Plastic`) false false))))

(fn `UserConstructionScript`)