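; Test robot assembled from part components such as floors, lidar, motors, wheels and arms; Tick only forces GlobalVariables.LevelPhase to 5.
; Per-part functions flag matching parts while left mouse targets a shelf object with their SDIndex, unless it is printed but not acided.
; SetAllVisibility shows each part if that flag or its Var is set.
; SetCollisions makes all parts blocking, simulating only FloorFirst; this file calls none of these functions.
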(event `self.ReceiveTick`
  (params (DeltaSeconds :type "Float (single-precision)"))
  (bind _asglobal_variables (cast `/Game/Workplace/Blueprints/GlobalVariables` (`GameplayStatics.GetGameInstance`)))
  (set `/Game/Workplace/Blueprints/GlobalVariables.LevelPhase` 5 _asglobal_variables))

(fn `Arm1Visibility`
  (bind _asglobal_variables (cast `/Game/Workplace/Blueprints/GlobalVariables` (`GameplayStatics.GetGameInstance`)))
  (if (`/Game/Workplace/Blueprints/GlobalVariables.LeftMousePressed` _asglobal_variables)
    (bind _asbp_shelf_objects (cast `/Game/Workplace/Blueprints/BP_Shelf_Objects` (`/Game/Workplace/Blueprints/GlobalVariables.HitResult` _asglobal_variables)))
    (if (== (`/Game/Workplace/Blueprints/BP_Shelf_Objects.SDIndex` _asbp_shelf_objects) 0)
      (if (`/Game/Workplace/Blueprints/BP_Shelf_Objects.Printed` _asbp_shelf_objects)
        (if (`/Game/Workplace/Blueprints/BP_Shelf_Objects.Acided` _asbp_shelf_objects)
          (set `self.Arm1Visible` true)
          (else
            (set `self.Arm1Visible` false)))
        (else
          (set `self.Arm1Visible` true))))
    (else
      (set `self.Arm1Visible` false))))

(fn `Arm2Visibility`
  (bind _asglobal_variables (cast `/Game/Workplace/Blueprints/GlobalVariables` (`GameplayStatics.GetGameInstance`)))
  (if (`/Game/Workplace/Blueprints/GlobalVariables.LeftMousePressed` _asglobal_variables)
    (bind _asbp_shelf_objects (cast `/Game/Workplace/Blueprints/BP_Shelf_Objects` (`/Game/Workplace/Blueprints/GlobalVariables.HitResult` _asglobal_variables)))
    (if (== (`/Game/Workplace/Blueprints/BP_Shelf_Objects.SDIndex` _asbp_shelf_objects) 0)
      (if (`/Game/Workplace/Blueprints/BP_Shelf_Objects.Printed` _asbp_shelf_objects)
        (if (`/Game/Workplace/Blueprints/BP_Shelf_Objects.Acided` _asbp_shelf_objects)
          (set `self.Arm2Visible` true)
          (else
            (set `self.Arm2Visible` false)))
        (else
          (set `self.Arm2Visible` true))))
    (else
      (set `self.Arm2Visible` false))))

(fn `Direction1Visibility`
  (bind _asglobal_variables (cast `/Game/Workplace/Blueprints/GlobalVariables` (`GameplayStatics.GetGameInstance`)))
  (if (`/Game/Workplace/Blueprints/GlobalVariables.LeftMousePressed` _asglobal_variables)
    (bind _asbp_shelf_objects (cast `/Game/Workplace/Blueprints/BP_Shelf_Objects` (`/Game/Workplace/Blueprints/GlobalVariables.HitResult` _asglobal_variables)))
    (if (== (`/Game/Workplace/Blueprints/BP_Shelf_Objects.SDIndex` _asbp_shelf_objects) 1)
      (if (`/Game/Workplace/Blueprints/BP_Shelf_Objects.Printed` _asbp_shelf_objects)
        (if (`/Game/Workplace/Blueprints/BP_Shelf_Objects.Acided` _asbp_shelf_objects)
          (set `self.Direction1Visible` true)
          (else
            (set `self.Direction1Visible` false)))
        (else
          (set `self.Direction1Visible` true))))
    (else
      (set `self.Direction1Visible` false))))

(fn `Direction2Visibility`
  (bind _asglobal_variables (cast `/Game/Workplace/Blueprints/GlobalVariables` (`GameplayStatics.GetGameInstance`)))
  (if (`/Game/Workplace/Blueprints/GlobalVariables.LeftMousePressed` _asglobal_variables)
    (bind _asbp_shelf_objects (cast `/Game/Workplace/Blueprints/BP_Shelf_Objects` (`/Game/Workplace/Blueprints/GlobalVariables.HitResult` _asglobal_variables)))
    (if (== (`/Game/Workplace/Blueprints/BP_Shelf_Objects.SDIndex` _asbp_shelf_objects) 1)
      (if (`/Game/Workplace/Blueprints/BP_Shelf_Objects.Printed` _asbp_shelf_objects)
        (if (`/Game/Workplace/Blueprints/BP_Shelf_Objects.Acided` _asbp_shelf_objects)
          (set `self.Direction2Visible` true)
          (else
            (set `self.Direction2Visible` false)))
        (else
          (set `self.Direction2Visible` true))))
    (else
      (set `self.Direction2Visible` false))))

(fn `Fastening1Visibility`
  (bind _asglobal_variables (cast `/Game/Workplace/Blueprints/GlobalVariables` (`GameplayStatics.GetGameInstance`)))
  (if (`/Game/Workplace/Blueprints/GlobalVariables.LeftMousePressed` _asglobal_variables)
    (bind _asbp_shelf_objects (cast `/Game/Workplace/Blueprints/BP_Shelf_Objects` (`/Game/Workplace/Blueprints/GlobalVariables.HitResult` _asglobal_variables)))
    (if (== (`/Game/Workplace/Blueprints/BP_Shelf_Objects.SDIndex` _asbp_shelf_objects) 2)
      (if (`/Game/Workplace/Blueprints/BP_Shelf_Objects.Printed` _asbp_shelf_objects)
        (if (`/Game/Workplace/Blueprints/BP_Shelf_Objects.Acided` _asbp_shelf_objects)
          (set `self.Fastening1Visible` true)
          (else
            (set `self.Fastening1Visible` false)))
        (else
          (set `self.Fastening1Visible` true))))
    (else
      (set `self.Fastening1Visible` false))))

(fn `Fastening2Visibility`
  (bind _asglobal_variables (cast `/Game/Workplace/Blueprints/GlobalVariables` (`GameplayStatics.GetGameInstance`)))
  (if (`/Game/Workplace/Blueprints/GlobalVariables.LeftMousePressed` _asglobal_variables)
    (bind _asbp_shelf_objects (cast `/Game/Workplace/Blueprints/BP_Shelf_Objects` (`/Game/Workplace/Blueprints/GlobalVariables.HitResult` _asglobal_variables)))
    (if (== (`/Game/Workplace/Blueprints/BP_Shelf_Objects.SDIndex` _asbp_shelf_objects) 2)
      (if (`/Game/Workplace/Blueprints/BP_Shelf_Objects.Printed` _asbp_shelf_objects)
        (if (`/Game/Workplace/Blueprints/BP_Shelf_Objects.Acided` _asbp_shelf_objects)
          (set `self.Fastening2Visible` true)
          (else
            (set `self.Fastening2Visible` false)))
        (else
          (set `self.Fastening2Visible` true))))
    (else
      (set `self.Fastening2Visible` false))))

(fn `Fastening3Visibility`
  (bind _asglobal_variables (cast `/Game/Workplace/Blueprints/GlobalVariables` (`GameplayStatics.GetGameInstance`)))
  (if (`/Game/Workplace/Blueprints/GlobalVariables.LeftMousePressed` _asglobal_variables)
    (bind _asbp_shelf_objects (cast `/Game/Workplace/Blueprints/BP_Shelf_Objects` (`/Game/Workplace/Blueprints/GlobalVariables.HitResult` _asglobal_variables)))
    (if (== (`/Game/Workplace/Blueprints/BP_Shelf_Objects.SDIndex` _asbp_shelf_objects) 2)
      (if (`/Game/Workplace/Blueprints/BP_Shelf_Objects.Printed` _asbp_shelf_objects)
        (if (`/Game/Workplace/Blueprints/BP_Shelf_Objects.Acided` _asbp_shelf_objects)
          (set `self.Fastening3Visible` true)
          (else
            (set `self.Fastening3Visible` false)))
        (else
          (set `self.Fastening3Visible` true))))
    (else
      (set `self.Fastening3Visible` false))))

(fn `Fastening4Visibility`
  (bind _asglobal_variables (cast `/Game/Workplace/Blueprints/GlobalVariables` (`GameplayStatics.GetGameInstance`)))
  (if (`/Game/Workplace/Blueprints/GlobalVariables.LeftMousePressed` _asglobal_variables)
    (bind _asbp_shelf_objects (cast `/Game/Workplace/Blueprints/BP_Shelf_Objects` (`/Game/Workplace/Blueprints/GlobalVariables.HitResult` _asglobal_variables)))
    (if (== (`/Game/Workplace/Blueprints/BP_Shelf_Objects.SDIndex` _asbp_shelf_objects) 2)
      (if (`/Game/Workplace/Blueprints/BP_Shelf_Objects.Printed` _asbp_shelf_objects)
        (if (`/Game/Workplace/Blueprints/BP_Shelf_Objects.Acided` _asbp_shelf_objects)
          (set `self.Fastening4Visible` true)
          (else
            (set `self.Fastening4Visible` false)))
        (else
          (set `self.Fastening4Visible` true))))
    (else
      (set `self.Fastening4Visible` false))))

(fn `FloorFirstVisibility`
  (bind _asglobal_variables (cast `/Game/Workplace/Blueprints/GlobalVariables` (`GameplayStatics.GetGameInstance`)))
  (if (`/Game/Workplace/Blueprints/GlobalVariables.LeftMousePressed` _asglobal_variables)
    (bind _asbp_shelf_objects (cast `/Game/Workplace/Blueprints/BP_Shelf_Objects` (`/Game/Workplace/Blueprints/GlobalVariables.HitResult` _asglobal_variables)))
    (if (== (`/Game/Workplace/Blueprints/BP_Shelf_Objects.SDIndex` _asbp_shelf_objects) 3)
      (if (`/Game/Workplace/Blueprints/BP_Shelf_Objects.Printed` _asbp_shelf_objects)
        (if (`/Game/Workplace/Blueprints/BP_Shelf_Objects.Acided` _asbp_shelf_objects)
          (set `self.FloorFirstVisible` true)
          (else
            (set `self.FloorFirstVisible` false)))
        (else
          (set `self.FloorFirstVisible` true))))
    (else
      (set `self.FloorFirstVisible` false))))

(fn `FloorSecondVisibility`
  (bind _asglobal_variables (cast `/Game/Workplace/Blueprints/GlobalVariables` (`GameplayStatics.GetGameInstance`)))
  (if (`/Game/Workplace/Blueprints/GlobalVariables.LeftMousePressed` _asglobal_variables)
    (bind _asbp_shelf_objects (cast `/Game/Workplace/Blueprints/BP_Shelf_Objects` (`/Game/Workplace/Blueprints/GlobalVariables.HitResult` _asglobal_variables)))
    (if (== (`/Game/Workplace/Blueprints/BP_Shelf_Objects.SDIndex` _asbp_shelf_objects) 4)
      (if (`/Game/Workplace/Blueprints/BP_Shelf_Objects.Printed` _asbp_shelf_objects)
        (if (`/Game/Workplace/Blueprints/BP_Shelf_Objects.Acided` _asbp_shelf_objects)
          (set `self.FloorSecondVisible` true)
          (else
            (set `self.FloorSecondVisible` false)))
        (else
          (set `self.FloorSecondVisible` true))))
    (else
      (set `self.FloorSecondVisible` false))))

(fn `LidarVisibility`
  (bind _asglobal_variables (cast `/Game/Workplace/Blueprints/GlobalVariables` (`GameplayStatics.GetGameInstance`)))
  (if (`/Game/Workplace/Blueprints/GlobalVariables.LeftMousePressed` _asglobal_variables)
    (bind _asbp_shelf_objects (cast `/Game/Workplace/Blueprints/BP_Shelf_Objects` (`/Game/Workplace/Blueprints/GlobalVariables.HitResult` _asglobal_variables)))
    (if (== (`/Game/Workplace/Blueprints/BP_Shelf_Objects.SDIndex` _asbp_shelf_objects) 5)
      (if (`/Game/Workplace/Blueprints/BP_Shelf_Objects.Printed` _asbp_shelf_objects)
        (if (`/Game/Workplace/Blueprints/BP_Shelf_Objects.Acided` _asbp_shelf_objects)
          (set `self.LidarVisible` true)
          (else
            (set `self.LidarVisible` false)))
        (else
          (set `self.LidarVisible` true))))
    (else
      (set `self.LidarVisible` false))))

(fn `Motor1Visibility`
  (bind _asglobal_variables (cast `/Game/Workplace/Blueprints/GlobalVariables` (`GameplayStatics.GetGameInstance`)))
  (if (`/Game/Workplace/Blueprints/GlobalVariables.LeftMousePressed` _asglobal_variables)
    (bind _asbp_shelf_objects (cast `/Game/Workplace/Blueprints/BP_Shelf_Objects` (`/Game/Workplace/Blueprints/GlobalVariables.HitResult` _asglobal_variables)))
    (if (== (`/Game/Workplace/Blueprints/BP_Shelf_Objects.SDIndex` _asbp_shelf_objects) 7)
      (if (`/Game/Workplace/Blueprints/BP_Shelf_Objects.Printed` _asbp_shelf_objects)
        (if (`/Game/Workplace/Blueprints/BP_Shelf_Objects.Acided` _asbp_shelf_objects)
          (set `self.Motor1Visible` true)
          (else
            (set `self.Motor1Visible` false)))
        (else
          (set `self.Motor1Visible` true))))
    (else
      (set `self.Motor1Visible` false))))

(fn `Motor2Visibility`
  (bind _asglobal_variables (cast `/Game/Workplace/Blueprints/GlobalVariables` (`GameplayStatics.GetGameInstance`)))
  (if (`/Game/Workplace/Blueprints/GlobalVariables.LeftMousePressed` _asglobal_variables)
    (bind _asbp_shelf_objects (cast `/Game/Workplace/Blueprints/BP_Shelf_Objects` (`/Game/Workplace/Blueprints/GlobalVariables.HitResult` _asglobal_variables)))
    (if (== (`/Game/Workplace/Blueprints/BP_Shelf_Objects.SDIndex` _asbp_shelf_objects) 7)
      (if (`/Game/Workplace/Blueprints/BP_Shelf_Objects.Printed` _asbp_shelf_objects)
        (if (`/Game/Workplace/Blueprints/BP_Shelf_Objects.Acided` _asbp_shelf_objects)
          (set `self.Motor2Visible` true)
          (else
            (set `self.Motor2Visible` false)))
        (else
          (set `self.Motor2Visible` true))))
    (else
      (set `self.Motor2Visible` false))))

(fn `MotorLock1Visibility`
  (bind _asglobal_variables (cast `/Game/Workplace/Blueprints/GlobalVariables` (`GameplayStatics.GetGameInstance`)))
  (if (`/Game/Workplace/Blueprints/GlobalVariables.LeftMousePressed` _asglobal_variables)
    (bind _asbp_shelf_objects (cast `/Game/Workplace/Blueprints/BP_Shelf_Objects` (`/Game/Workplace/Blueprints/GlobalVariables.HitResult` _asglobal_variables)))
    (if (== (`/Game/Workplace/Blueprints/BP_Shelf_Objects.SDIndex` _asbp_shelf_objects) 6)
      (if (`/Game/Workplace/Blueprints/BP_Shelf_Objects.Printed` _asbp_shelf_objects)
        (if (`/Game/Workplace/Blueprints/BP_Shelf_Objects.Acided` _asbp_shelf_objects)
          (set `self.MotorLock1Visible` true)
          (else
            (set `self.MotorLock1Visible` false)))
        (else
          (set `self.MotorLock1Visible` true))))
    (else
      (set `self.MotorLock1Visible` false))))

(fn `MotorLock2Visibility`
  (bind _asglobal_variables (cast `/Game/Workplace/Blueprints/GlobalVariables` (`GameplayStatics.GetGameInstance`)))
  (if (`/Game/Workplace/Blueprints/GlobalVariables.LeftMousePressed` _asglobal_variables)
    (bind _asbp_shelf_objects (cast `/Game/Workplace/Blueprints/BP_Shelf_Objects` (`/Game/Workplace/Blueprints/GlobalVariables.HitResult` _asglobal_variables)))
    (if (== (`/Game/Workplace/Blueprints/BP_Shelf_Objects.SDIndex` _asbp_shelf_objects) 6)
      (if (`/Game/Workplace/Blueprints/BP_Shelf_Objects.Printed` _asbp_shelf_objects)
        (if (`/Game/Workplace/Blueprints/BP_Shelf_Objects.Acided` _asbp_shelf_objects)
          (set `self.MotorLock2Visible` true)
          (else
            (set `self.MotorLock2Visible` false)))
        (else
          (set `self.MotorLock2Visible` true))))
    (else
      (set `self.MotorLock2Visible` false))))

(fn `SetAllVisibility`
  (`SceneComponent.SetVisibility` (`self.FloorFirst`) (or (`self.FloorFirstVisible`) (`self.FloorFirstVar`)) false)
  (`SceneComponent.SetVisibility` (`self.FloorSecond`) (or (`self.FloorSecondVisible`) (`self.FloorSecondVar`)) false)
  (`SceneComponent.SetVisibility` (`self.Lidar`) (or (`self.LidarVisible`) (`self.LidarVar`)) false)
  (`SceneComponent.SetVisibility` (`self.MotorLock1`) (or (`self.MotorLock1Visible`) (`self.MotorLock1Var`)) false)
  (`SceneComponent.SetVisibility` (`self.MotorLock2`) (or (`self.MotorLock2Visible`) (`self.MotorLock2Var`)) false)
  (`SceneComponent.SetVisibility` (`self.Motor1`) (or (`self.Motor1Visible`) (`self.Motor1Var`)) false)
  (`SceneComponent.SetVisibility` (`self.Motor2`) (or (`self.Motor2Visible`) (`self.Motor2Var`)) false)
  (`SceneComponent.SetVisibility` (`self.Wheel1`) (or (`self.Wheel1Visible`) (`self.Wheel1Var`)) false)
  (`SceneComponent.SetVisibility` (`self.Wheel2`) (or (`self.Wheel2Visible`) (`self.Wheel2Var`)) false)
  (`SceneComponent.SetVisibility` (`self.Direction1`) (or (`self.Direction1Visible`) (`self.Direction1Var`)) false)
  (`SceneComponent.SetVisibility` (`self.Fastening1`) (or (`self.Fastening1Visible`) (`self.Fastening1Var`)) false)
  (`SceneComponent.SetVisibility` (`self.Fastening2`) (or (`self.Fastening2Visible`) (`self.Fastening2Var`)) false)
  (`SceneComponent.SetVisibility` (`self.Direction2`) (or (`self.Direction2Visible`) (`self.Direction2Var`)) false)
  (`SceneComponent.SetVisibility` (`self.Arm1`) (or (`self.Arm1Visible`) (`self.Arm1Var`)) false)
  (`SceneComponent.SetVisibility` (`self.Arm2`) (or (`self.Arm2Visible`) (`self.Arm2Var`)) false)
  (`SceneComponent.SetVisibility` (`self.Fastening3`) (or (`self.Fastening3Visible`) (`self.Fastening3Var`)) false)
  (`SceneComponent.SetVisibility` (`self.Fastening4`) (or (`self.Fastening4Visible`) (`self.Fastening4Var`)) false))

(fn `SetCollisions`
  (bind _floorfirst (`self.FloorFirst`))
  (bind _floorsecond (`self.FloorSecond`))
  (bind _lidar (`self.Lidar`))
  (bind _motorlock1 (`self.MotorLock1`))
  (bind _motorlock2 (`self.MotorLock2`))
  (bind _motor1 (`self.Motor1`))
  (bind _motor2 (`self.Motor2`))
  (bind _wheel1 (`self.Wheel1`))
  (bind _wheel2 (`self.Wheel2`))
  (bind _direction1 (`self.Direction1`))
  (bind _fastening1 (`self.Fastening1`))
  (bind _fastening2 (`self.Fastening2`))
  (bind _direction2 (`self.Direction2`))
  (bind _arm1 (`self.Arm1`))
  (bind _arm2 (`self.Arm2`))
  (bind _fastening3 (`self.Fastening3`))
  (bind _fastening4 (`self.Fastening4`))
  (`PrimitiveComponent.SetSimulatePhysics` _floorfirst true)
  (`PrimitiveComponent.SetCollisionResponseToAllChannels` _floorfirst "ECR_Block")
  (`PrimitiveComponent.SetCollisionEnabled` _floorfirst "QueryAndPhysics")
  (`PrimitiveComponent.SetCollisionObjectType` _floorfirst "ECC_PhysicsBody")
  (`PrimitiveComponent.SetSimulatePhysics` _floorsecond false)
  (`PrimitiveComponent.SetCollisionResponseToAllChannels` _floorsecond "ECR_Block")
  (`PrimitiveComponent.SetCollisionEnabled` _floorsecond "QueryAndPhysics")
  (`PrimitiveComponent.SetCollisionObjectType` _floorsecond "ECC_PhysicsBody")
  (`PrimitiveComponent.SetSimulatePhysics` _lidar false)
  (`PrimitiveComponent.SetCollisionResponseToAllChannels` _lidar "ECR_Block")
  (`PrimitiveComponent.SetCollisionEnabled` _lidar "QueryAndPhysics")
  (`PrimitiveComponent.SetCollisionObjectType` _lidar "ECC_PhysicsBody")
  (`PrimitiveComponent.SetSimulatePhysics` _motorlock1 false)
  (`PrimitiveComponent.SetCollisionResponseToAllChannels` _motorlock1 "ECR_Block")
  (`PrimitiveComponent.SetCollisionEnabled` _motorlock1 "QueryAndPhysics")
  (`PrimitiveComponent.SetCollisionObjectType` _motorlock1 "ECC_PhysicsBody")
  (`PrimitiveComponent.SetSimulatePhysics` _motorlock2 false)
  (`PrimitiveComponent.SetCollisionResponseToAllChannels` _motorlock2 "ECR_Block")
  (`PrimitiveComponent.SetCollisionEnabled` _motorlock2 "QueryAndPhysics")
  (`PrimitiveComponent.SetCollisionObjectType` _motorlock2 "ECC_PhysicsBody")
  (`PrimitiveComponent.SetSimulatePhysics` _motor1 false)
  (`PrimitiveComponent.SetCollisionResponseToAllChannels` _motor1 "ECR_Block")
  (`PrimitiveComponent.SetCollisionEnabled` _motor1 "QueryAndPhysics")
  (`PrimitiveComponent.SetCollisionObjectType` _motor1 "ECC_PhysicsBody")
  (`PrimitiveComponent.SetSimulatePhysics` _motor2 false)
  (`PrimitiveComponent.SetCollisionResponseToAllChannels` _motor2 "ECR_Block")
  (`PrimitiveComponent.SetCollisionEnabled` _motor2 "QueryAndPhysics")
  (`PrimitiveComponent.SetCollisionObjectType` _motor2 "ECC_PhysicsBody")
  (`PrimitiveComponent.SetSimulatePhysics` _wheel1 false)
  (`PrimitiveComponent.SetCollisionResponseToAllChannels` _wheel1 "ECR_Block")
  (`PrimitiveComponent.SetCollisionEnabled` _wheel1 "QueryAndPhysics")
  (`PrimitiveComponent.SetCollisionObjectType` _wheel1 "ECC_PhysicsBody")
  (`PrimitiveComponent.SetSimulatePhysics` _wheel2 false)
  (`PrimitiveComponent.SetCollisionResponseToAllChannels` _wheel2 "ECR_Block")
  (`PrimitiveComponent.SetCollisionEnabled` _wheel2 "QueryAndPhysics")
  (`PrimitiveComponent.SetCollisionObjectType` _wheel2 "ECC_PhysicsBody")
  (`PrimitiveComponent.SetSimulatePhysics` _direction1 false)
  (`PrimitiveComponent.SetCollisionResponseToAllChannels` _direction1 "ECR_Block")
  (`PrimitiveComponent.SetCollisionEnabled` _direction1 "QueryAndPhysics")
  (`PrimitiveComponent.SetCollisionObjectType` _direction1 "ECC_PhysicsBody")
  (`PrimitiveComponent.SetSimulatePhysics` _fastening1 false)
  (`PrimitiveComponent.SetCollisionResponseToAllChannels` _fastening1 "ECR_Block")
  (`PrimitiveComponent.SetCollisionEnabled` _fastening1 "QueryAndPhysics")
  (`PrimitiveComponent.SetCollisionObjectType` _fastening1 "ECC_PhysicsBody")
  (`PrimitiveComponent.SetSimulatePhysics` _fastening2 false)
  (`PrimitiveComponent.SetCollisionResponseToAllChannels` _fastening2 "ECR_Block")
  (`PrimitiveComponent.SetCollisionEnabled` _fastening2 "QueryAndPhysics")
  (`PrimitiveComponent.SetCollisionObjectType` _fastening2 "ECC_PhysicsBody")
  (`PrimitiveComponent.SetSimulatePhysics` _direction2 false)
  (`PrimitiveComponent.SetCollisionResponseToAllChannels` _direction2 "ECR_Block")
  (`PrimitiveComponent.SetCollisionEnabled` _direction2 "QueryAndPhysics")
  (`PrimitiveComponent.SetCollisionObjectType` _direction2 "ECC_PhysicsBody")
  (`PrimitiveComponent.SetSimulatePhysics` _arm1 false)
  (`PrimitiveComponent.SetCollisionResponseToAllChannels` _arm1 "ECR_Block")
  (`PrimitiveComponent.SetCollisionEnabled` _arm1 "QueryAndPhysics")
  (`PrimitiveComponent.SetCollisionObjectType` _arm1 "ECC_PhysicsBody")
  (`PrimitiveComponent.SetSimulatePhysics` _arm2 false)
  (`PrimitiveComponent.SetCollisionResponseToAllChannels` _arm2 "ECR_Block")
  (`PrimitiveComponent.SetCollisionEnabled` _arm2 "QueryAndPhysics")
  (`PrimitiveComponent.SetCollisionObjectType` _arm2 "ECC_PhysicsBody")
  (`PrimitiveComponent.SetSimulatePhysics` _fastening3 false)
  (`PrimitiveComponent.SetCollisionResponseToAllChannels` _fastening3 "ECR_Block")
  (`PrimitiveComponent.SetCollisionEnabled` _fastening3 "QueryAndPhysics")
  (`PrimitiveComponent.SetCollisionObjectType` _fastening3 "ECC_PhysicsBody")
  (`PrimitiveComponent.SetSimulatePhysics` _fastening4 false)
  (`PrimitiveComponent.SetCollisionResponseToAllChannels` _fastening4 "ECR_Block")
  (`PrimitiveComponent.SetCollisionEnabled` _fastening4 "QueryAndPhysics")
  (`PrimitiveComponent.SetCollisionObjectType` _fastening4 "ECC_PhysicsBody"))

(fn `UserConstructionScript`)

(fn `Wheel1Visibility`
  (bind _asglobal_variables (cast `/Game/Workplace/Blueprints/GlobalVariables` (`GameplayStatics.GetGameInstance`)))
  (if (`/Game/Workplace/Blueprints/GlobalVariables.LeftMousePressed` _asglobal_variables)
    (bind _asbp_shelf_objects (cast `/Game/Workplace/Blueprints/BP_Shelf_Objects` (`/Game/Workplace/Blueprints/GlobalVariables.HitResult` _asglobal_variables)))
    (if (== (`/Game/Workplace/Blueprints/BP_Shelf_Objects.SDIndex` _asbp_shelf_objects) 8)
      (if (`/Game/Workplace/Blueprints/BP_Shelf_Objects.Printed` _asbp_shelf_objects)
        (if (`/Game/Workplace/Blueprints/BP_Shelf_Objects.Acided` _asbp_shelf_objects)
          (set `self.Wheel1Visible` true)
          (else
            (set `self.Wheel1Visible` false)))
        (else
          (set `self.Wheel1Visible` true))))
    (else
      (set `self.Wheel1Visible` false))))

(fn `Wheel2Visibility`
  (bind _asglobal_variables (cast `/Game/Workplace/Blueprints/GlobalVariables` (`GameplayStatics.GetGameInstance`)))
  (if (`/Game/Workplace/Blueprints/GlobalVariables.LeftMousePressed` _asglobal_variables)
    (bind _asbp_shelf_objects (cast `/Game/Workplace/Blueprints/BP_Shelf_Objects` (`/Game/Workplace/Blueprints/GlobalVariables.HitResult` _asglobal_variables)))
    (if (== (`/Game/Workplace/Blueprints/BP_Shelf_Objects.SDIndex` _asbp_shelf_objects) 8)
      (if (`/Game/Workplace/Blueprints/BP_Shelf_Objects.Printed` _asbp_shelf_objects)
        (if (`/Game/Workplace/Blueprints/BP_Shelf_Objects.Acided` _asbp_shelf_objects)
          (set `self.Wheel2Visible` true)
          (else
            (set `self.Wheel2Visible` false)))
        (else
          (set `self.Wheel2Visible` true))))
    (else
      (set `self.Wheel2Visible` false))))