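; Track actor that reveals its eleven object components one at a time, driven by an index in the game instance.
; BeginPlay hides all of them and disables their collision.
; Each Tick reads TrackObjectsVisibleIndex from GlobalVariables and shows the matching object with collision, never re-hiding earlier ones.
; Revealing the last object also sets the game instance's LevelPhase to 3.
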(event `self.ReceiveBeginPlay`
  (bind _object5 (`self.Object5`))
  (bind _object6 (`self.Object6`))
  (bind _object7 (`self.Object7`))
  (bind _object8 (`self.Object8`))
  (bind _object9 (`self.Object9`))
  (bind _object10 (`self.Object10`))
  (bind _object11 (`self.Object11`))
  (bind _object1 (`self.Object1`))
  (bind _object2 (`self.Object2`))
  (bind _object3 (`self.Object3`))
  (bind _object4 (`self.Object4`))
  (`|ExecutionSequence`
    (:`then_0`
      ;[1 1 1] Задание невидимости объектов
      (`PrimitiveComponent.SetCollisionEnabled` _object1 "NoCollision")
      (`SceneComponent.SetVisibility` _object1 false false))
    (:`then_1`
      (`PrimitiveComponent.SetCollisionEnabled` _object2 "NoCollision")
      (`SceneComponent.SetVisibility` _object2 false false))
    (:`then_2`
      (`PrimitiveComponent.SetCollisionEnabled` _object3 "NoCollision")
      (`SceneComponent.SetVisibility` _object3 false false))
    (:`then_3`
      (`PrimitiveComponent.SetCollisionEnabled` _object4 "NoCollision")
      (`SceneComponent.SetVisibility` _object4 false false))
    (:`then_4`
      (`PrimitiveComponent.SetCollisionEnabled` _object5 "NoCollision")
      (`SceneComponent.SetVisibility` _object5 false false))
    (:`then_5`
      (`PrimitiveComponent.SetCollisionEnabled` _object6 "NoCollision")
      (`SceneComponent.SetVisibility` _object6 false false))
    (:`then_6`
      (`PrimitiveComponent.SetCollisionEnabled` _object7 "NoCollision")
      (`SceneComponent.SetVisibility` _object7 false false))
    (:`then_7`
      (`PrimitiveComponent.SetCollisionEnabled` _object8 "NoCollision")
      (`SceneComponent.SetVisibility` _object8 false false))
    (:`then_8`
      (`PrimitiveComponent.SetCollisionEnabled` _object9 "NoCollision")
      (`SceneComponent.SetVisibility` _object9 false false))
    (:`then_9`
      (`PrimitiveComponent.SetCollisionEnabled` _object10 "NoCollision")
      (`SceneComponent.SetVisibility` _object10 false false))
    (:`then_10`
      (`PrimitiveComponent.SetCollisionEnabled` _object11 "NoCollision")
      (`SceneComponent.SetVisibility` _object11 false false))
    (:`then_11`
      (set `self.ObjectIndex` -1))))

(event `self.ReceiveTick`
  (params (DeltaSeconds :type "Float (single-precision)"))
  (bind _object1 (`self.Object1`))
  (bind _object2 (`self.Object2`))
  (bind _object3 (`self.Object3`))
  (bind _object4 (`self.Object4`))
  (bind _object5 (`self.Object5`))
  (bind _object6 (`self.Object6`))
  (bind _object7 (`self.Object7`))
  (bind _object8 (`self.Object8`))
  (bind _object9 (`self.Object9`))
  (bind _object10 (`self.Object10`))
  (bind _object11 (`self.Object11`))
  (bind _asglobal_variables (cast `/Game/Workplace/Blueprints/GlobalVariables` (`GameplayStatics.GetGameInstance`)))
  (set `self.ObjectIndex` (`/Game/Workplace/Blueprints/GlobalVariables.TrackObjectsVisibleIndex` _asglobal_variables))
  (`|ExecutionSequence`
    (:`then_0`
      (if (== (`self.ObjectIndex`) 0)
        (`PrimitiveComponent.SetCollisionEnabled` _object1 "QueryAndPhysics")
        (`SceneComponent.SetVisibility` _object1 true false)))
    (:`then_1`
      (if (== (`self.ObjectIndex`) 1)
        (`PrimitiveComponent.SetCollisionEnabled` _object2 "QueryAndPhysics")
        (`SceneComponent.SetVisibility` _object2 true false)))
    (:`then_2`
      (if (== (`self.ObjectIndex`) 2)
        (`PrimitiveComponent.SetCollisionEnabled` _object3 "QueryAndPhysics")
        (`SceneComponent.SetVisibility` _object3 true false)))
    (:`then_3`
      (if (== (`self.ObjectIndex`) 3)
        (`PrimitiveComponent.SetCollisionEnabled` _object4 "QueryAndPhysics")
        (`SceneComponent.SetVisibility` _object4 true false)))
    (:`then_4`
      (if (== (`self.ObjectIndex`) 4)
        (`PrimitiveComponent.SetCollisionEnabled` _object5 "QueryAndPhysics")
        (`SceneComponent.SetVisibility` _object5 true false)))
    (:`then_5`
      (if (== (`self.ObjectIndex`) 5)
        (`PrimitiveComponent.SetCollisionEnabled` _object6 "QueryAndPhysics")
        (`SceneComponent.SetVisibility` _object6 true false)))
    (:`then_6`
      (if (== (`self.ObjectIndex`) 6)
        (`PrimitiveComponent.SetCollisionEnabled` _object7 "QueryAndPhysics")
        (`SceneComponent.SetVisibility` _object7 true false)))
    (:`then_7`
      (if (== (`self.ObjectIndex`) 7)
        (`PrimitiveComponent.SetCollisionEnabled` _object8 "QueryAndPhysics")
        (`SceneComponent.SetVisibility` _object8 true false)))
    (:`then_8`
      (if (== (`self.ObjectIndex`) 8)
        (`PrimitiveComponent.SetCollisionEnabled` _object9 "QueryAndPhysics")
        (`SceneComponent.SetVisibility` _object9 true false)))
    (:`then_9`
      (if (== (`self.ObjectIndex`) 9)
        (`PrimitiveComponent.SetCollisionEnabled` _object10 "QueryAndPhysics")
        (`SceneComponent.SetVisibility` _object10 true false)))
    (:`then_10`
      (if (== (`self.ObjectIndex`) 10)
        (`PrimitiveComponent.SetCollisionEnabled` _object11 "QueryAndPhysics")
        (`SceneComponent.SetVisibility` _object11 true false)
        (bind _asglobal_variables_2 (cast `/Game/Workplace/Blueprints/GlobalVariables` (`GameplayStatics.GetGameInstance`)))
        (set `/Game/Workplace/Blueprints/GlobalVariables.LevelPhase` 3 _asglobal_variables_2)))))

(fn `UserConstructionScript`)