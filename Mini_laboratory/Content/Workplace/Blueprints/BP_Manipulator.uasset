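; Workplace robotic manipulator that plays take and drop sequences to move an object into a printed box.
; The Mode event runs chained timelines that write bone values into ABP_Manipulator.
; Between drop phases it messages box actors with material and SD index; after a take it broadcasts MoveBack.
; The held object is a socket-attached component shown on Tick from a GameInstance flag, and finishing a drop clears the busy flag.
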(event `self.ReceiveTick`
  (params (DeltaSeconds :type "Float (single-precision)"))
  ;[1 1 1] Задаем видимость
  (bind _asglobal_variables (cast `/Game/Workplace/Blueprints/GlobalVariables` (`GameplayStatics.GetGameInstance`)))
  (`SceneComponent.SetVisibility` (`self.Object`) (`/Game/Workplace/Blueprints/GlobalVariables.ManipulatorTakeObject` _asglobal_variables) false))

(event `self.ReceiveBeginPlay`
  ;[1 1 1] Закрепляем позицию объекта
  (`SceneComponent.K2_AttachToComponent` (`self.Object`) (`self.Manipulator`) "Object" "KeepRelative" "KeepRelative" "KeepWorld" true)
  (set `self.SavedMode` "")
  (set `self.SDIndex` 0)
  (set `self.Material` null))

(event `/Game/Workplace/Blueprints/BI_Manipulator.Mode`
  (params (Mode :type Text) (SDIndex :type Integer) (Material :type "Material Object Reference"))
  (set `self.Material` Material)
  (set `self.SDIndex` SDIndex)
  (bind _output_get (set `self.SavedMode` Mode))
  (`|ExecutionSequence`
    (:`then_0`
      ;[1 1 1] Положить объект в коробку
      (if (`KismetTextLibrary.EqualEqual_TextText` _output_get (`|FormatText` "Drop"))
        (bind _animation (`self.GetAnimation`))
        (set `/Game/Workplace/Animations/ABP_Manipulator.DropObject` true _animation)
        (bind (_direction _bone _bone_002 _bone_006 _bone_007 _bone_001) (`Timeline|DropObject1` :!via `PlayFromStart`)
          (:`Update`
            (set `/Game/Workplace/Animations/ABP_Manipulator.Bone` _bone _animation)
            (set `/Game/Workplace/Animations/ABP_Manipulator.Bone_001` _bone_001 _animation)
            (set `/Game/Workplace/Animations/ABP_Manipulator.Bone_002` _bone_002 _animation)
            (set `/Game/Workplace/Animations/ABP_Manipulator.Bone_006` _bone_006 _animation)
            (set `/Game/Workplace/Animations/ABP_Manipulator.Bone_007` _bone_007 _animation))
          (:`Finished`
            (bind _asglobal_variables (cast `/Game/Workplace/Blueprints/GlobalVariables` (`GameplayStatics.GetGameInstance`)))
            (set `/Game/Workplace/Blueprints/GlobalVariables.ManipulatorTakeObject` false _asglobal_variables)
            (bind _outactors (`GameplayStatics.GetAllActorsWithInterface` "/Game/Workplace/Blueprints/BI_Drop_In_Printed_Box.BI_Drop_In_Printed_Box_C"))
            (message `/Game/Workplace/Blueprints/BI_Drop_In_Printed_Box.DropObjectInBox` _outactors (`self.Material`) (`self.SDIndex`))
            (bind _animation_2 (`self.GetAnimation`))
            (bind (_direction_2 _bone_2 _bone_002_2 _bone_006_2 _bone_007_2 _bone_001_2) (`Timeline|DropObject2` :!via `PlayFromStart`)
              (:`Update`
                (set `/Game/Workplace/Animations/ABP_Manipulator.Bone` _bone_2 _animation_2)
                (set `/Game/Workplace/Animations/ABP_Manipulator.Bone_001` _bone_001_2 _animation_2)
                (set `/Game/Workplace/Animations/ABP_Manipulator.Bone_002` _bone_002_2 _animation_2)
                (set `/Game/Workplace/Animations/ABP_Manipulator.Bone_006` _bone_006_2 _animation_2)
                (set `/Game/Workplace/Animations/ABP_Manipulator.Bone_007` _bone_007_2 _animation_2))
              (:`Finished`
                (set `/Game/Workplace/Animations/ABP_Manipulator.Completed` true _animation_2)
                (bind _asglobal_variables_2 (cast `/Game/Workplace/Blueprints/GlobalVariables` (`GameplayStatics.GetGameInstance`)))
                (set `/Game/Workplace/Blueprints/GlobalVariables.ManipulatorBusy` false _asglobal_variables_2)))))))
    (:`then_1`
      ;[1 1 1] Захват объекта
      (if (`KismetTextLibrary.EqualEqual_TextText` _output_get (`|FormatText` "Take"))
        (bind _animation_3 (`self.GetAnimation`))
        (set `/Game/Workplace/Animations/ABP_Manipulator.TakeObject` true _animation_3)
        (bind (_direction_3 _bone_001_3 _bone_002_3 _bone_003 _bone_006_3 _bone_007_3) (`Timeline|TakeObject1` :!via `PlayFromStart`)
          (:`Update`
            (set `/Game/Workplace/Animations/ABP_Manipulator.Bone_001` _bone_001_3 _animation_3)
            (set `/Game/Workplace/Animations/ABP_Manipulator.Bone_002` _bone_002_3 _animation_3)
            (set `/Game/Workplace/Animations/ABP_Manipulator.Bone_003` _bone_003 _animation_3)
            (set `/Game/Workplace/Animations/ABP_Manipulator.Bone_006` _bone_006_3 _animation_3)
            (set `/Game/Workplace/Animations/ABP_Manipulator.Bone_007` _bone_007_3 _animation_3))
          (:`Finished`
            (bind _asglobal_variables_3 (cast `/Game/Workplace/Blueprints/GlobalVariables` (`GameplayStatics.GetGameInstance`)))
            (set `/Game/Workplace/Blueprints/GlobalVariables.ManipulatorTakeObject` true _asglobal_variables_3)
            (bind _animation_4 (`self.GetAnimation`))
            (bind (_direction_4 _bone_001_4 _bone_002_4 _bone_003_2 _bone_006_4 _bone_007_4) (`Timeline|TakeObject2` :!via `PlayFromStart`)
              (:`Update`
                (set `/Game/Workplace/Animations/ABP_Manipulator.Bone_001` _bone_001_4 _animation_4)
                (set `/Game/Workplace/Animations/ABP_Manipulator.Bone_002` _bone_002_4 _animation_4)
                (set `/Game/Workplace/Animations/ABP_Manipulator.Bone_003` _bone_003_2 _animation_4)
                (set `/Game/Workplace/Animations/ABP_Manipulator.Bone_006` _bone_006_4 _animation_4)
                (set `/Game/Workplace/Animations/ABP_Manipulator.Bone_007` _bone_007_4 _animation_4))
              (:`Finished`
                (set `/Game/Workplace/Animations/ABP_Manipulator.Completed` true _animation_4)
                (bind _outactors_2 (`GameplayStatics.GetAllActorsWithInterface` "/Game/Workplace/Blueprints/BI_MoveBack.BI_MoveBack_C"))
                (message `/Game/Workplace/Blueprints/BI_MoveBack.MoveBack` _outactors_2)))))))))

(fn `GetAnimation`
  (returns (Animation :type "/Game/Workplace/Animations/ABP_Manipulator Object Reference"))
  (bind _asabp_manipulator (cast `/Game/Workplace/Animations/ABP_Manipulator` (`SkeletalMeshComponent.GetAnimInstance` (`self.Manipulator`))))
  (return _asabp_manipulator))

(fn `UserConstructionScript`)