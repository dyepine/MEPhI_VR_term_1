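; Workplace 3D printer actor that prints SD-card objects with a colored spool and button press from level phase 3.
; Overlapping spools sets the plastic material and ejects the previous one.
; Tick polls state, driving bulb, button and AnimBP phases; infill and support set print speed, which weights random failure.
; Successful prints take mesh and transform from GlobalVariables, then signal the shared manipulator by interface, guarded by a busy flag.
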(event `self.ReceiveBeginPlay`
  (bind _asabp_3d_printer_up (cast `/Game/Workplace/Animations/ABP_3D_Printer_UP` (`SkeletalMeshComponent.GetAnimInstance` (`self.Printer`))))
  (set `/Game/Workplace/Animations/ABP_3D_Printer_UP.Speed` 0.0 _asabp_3d_printer_up)
  (set `self.Print` false)
  (set `self.SpoolAdded` false)
  (set `self.SDFilling` 0)
  (set `self.SDSupport` false)
  (bind _asglobal_variables (cast `/Game/Workplace/Blueprints/GlobalVariables` (`GameplayStatics.GetGameInstance`)))
  (set `self.MaxSpeed` (`/Game/Workplace/Blueprints/GlobalVariables.MaxPrintSpeed` _asglobal_variables))
  (set `self.Broke` false)
  (set `self.ThisPrinterUsed` false))

(event `self.HolderCollision.OnComponentBeginOverlap`
  (params (OverlappedComponent :type "PrimitiveComponent Object Reference") (OtherActor :type "Actor Object Reference") (OtherComp :type "PrimitiveComponent Object Reference") (OtherBodyIndex :type Integer) (bFromSweep :type Boolean) (SweepResult :type "HitResult Structure (by ref)"))
  ;[1 1 1] Меняем бобины
  (if (not (`self.Print`))
    (`|ExecutionSequence`
      (:`then_0`
        (`self.ChangeRedSpool` OtherActor))
      (:`then_1`
        (`self.ChangeYellowSpool` OtherActor))
      (:`then_2`
        (`self.ChangeGreenSpool` OtherActor))
      (:`then_3`
        (`self.ChangeBlueSpool` OtherActor)))
    (set `self.SpoolAdded` true)))

(event `self.ReceiveTick`
  (params (DeltaSeconds :type "Float (single-precision)"))
  (bind _maxspeed (`self.MaxSpeed`))
  (bind _maxspeed_2 (`self.MaxSpeed`))
  (`|ExecutionSequence`
    (:`then_0`
      ;[1 1 1] Проверка фазы
      (bind _asglobal_variables (cast `/Game/Workplace/Blueprints/GlobalVariables` (`GameplayStatics.GetGameInstance`)))
      (if (>= (`/Game/Workplace/Blueprints/GlobalVariables.LevelPhase` _asglobal_variables) 3)
        (if (`self.Print`)
          ;[1 1 1] Идет печать
          (bind _asabp_3d_printer_up (cast `/Game/Workplace/Animations/ABP_3D_Printer_UP` (`SkeletalMeshComponent.GetAnimInstance` (`self.Printer`))))
          (if (`/Game/Workplace/Animations/ABP_3D_Printer_UP.Phase2` _asabp_3d_printer_up)
            ;[1 1 1] Проверяем на ошибку печати
            (if (`self.Broke`)
              ;[1 1 1] Деталь сломалась
              (bind _asbp_button (cast `/Game/Workplace/Blueprints/BP_Button` (`ChildActorComponent.ChildActor` (`self.Button`))))
              (set `/Game/Workplace/Blueprints/BP_Button.State` true _asbp_button)
              (set `/Game/Workplace/Blueprints/BP_Button.PreState` true _asbp_button)
              (bind _asabp_3d_printer_up_2 (cast `/Game/Workplace/Animations/ABP_3D_Printer_UP` (`SkeletalMeshComponent.GetAnimInstance` (`self.Printer`))))
              (set `/Game/Workplace/Animations/ABP_3D_Printer_UP.Phase3` true _asabp_3d_printer_up_2)
              (`PrimitiveComponent.SetMaterial` (`self.Bulb`) 0 "/Game/Workplace/Materials/M_Glow_Green.M_Glow_Green")
              (bind _asbp_button_2 (cast `/Game/Workplace/Blueprints/BP_Button` (`ChildActorComponent.ChildActor` (`self.Button`))))
              (set `/Game/Workplace/Blueprints/BP_Button.State` false _asbp_button_2)
              (set `/Game/Workplace/Blueprints/BP_Button.PreState` false _asbp_button_2)
              (set `self.Broke` false)
              (set `self.Print` false)
              (else
                ;[1 1 1] Задаем объект напечатенный
                (bind _asglobal_variables_2 (cast `/Game/Workplace/Blueprints/GlobalVariables` (`GameplayStatics.GetGameInstance`)))
                (`StaticMeshComponent.SetStaticMesh` (`self.PrintedObject`) (`|GetArrayItem` (`/Game/Workplace/Blueprints/GlobalVariables.SDObjects` _asglobal_variables_2) (`self.SDIndex`)))
                (bind _asbp_empty_spool (cast `/Game/Workplace/Blueprints/BP_Empty_Spool` (`ChildActorComponent.ChildActor` (`self.Spool`))))
                (bind _asmaterial (cast `Material` (`PrimitiveComponent.GetMaterial` (`/Game/Workplace/Blueprints/BP_Empty_Spool.Plastic` _asbp_empty_spool) 0)))
                (`PrimitiveComponent.SetMaterial` (`self.PrintedObject`) 0 _asmaterial)
                (bind _asglobal_variables_3 (cast `/Game/Workplace/Blueprints/GlobalVariables` (`GameplayStatics.GetGameInstance`)))
                (`SceneComponent.K2_SetWorldRotation` (`self.PrintedObject`) (`KismetMathLibrary.Conv_VectorToRotator` (`|GetArrayItem` (`/Game/Workplace/Blueprints/GlobalVariables.SDObjectsRotation` _asglobal_variables_3) (`self.SDIndex`))) false false)
                (bind _asglobal_variables_4 (cast `/Game/Workplace/Blueprints/GlobalVariables` (`GameplayStatics.GetGameInstance`)))
                (`SceneComponent.SetWorldScale3D` (`self.PrintedObject`) (`KismetMathLibrary.Conv_DoubleToVector` (`|GetArrayItem` (`/Game/Workplace/Blueprints/GlobalVariables.SDObjectsScale` _asglobal_variables_4) (`self.SDIndex`))))
                ;[1 1 1] Отправка команды на захват объекта
                (bind _asglobal_variables_5 (cast `/Game/Workplace/Blueprints/GlobalVariables` (`GameplayStatics.GetGameInstance`)))
                (if (`/Game/Workplace/Blueprints/GlobalVariables.ManipulatorBusy` _asglobal_variables_5)
                  ;[1 1 1] Окончание печати
                  (if (`self.ThisPrinterUsed`)
                    (bind _asglobal_variables_6 (cast `/Game/Workplace/Blueprints/GlobalVariables` (`GameplayStatics.GetGameInstance`)))
                    (if (`/Game/Workplace/Blueprints/GlobalVariables.ManipulatorTakeObject` _asglobal_variables_6)
                      (`SceneComponent.SetWorldScale3D` (`self.PrintedObject`) (0.0 0.0 0.0))
                      (bind _asabp_3d_printer_up_3 (cast `/Game/Workplace/Animations/ABP_3D_Printer_UP` (`SkeletalMeshComponent.GetAnimInstance` (`self.Printer`))))
                      (set `/Game/Workplace/Animations/ABP_3D_Printer_UP.Phase3` true _asabp_3d_printer_up_3)
                      (`PrimitiveComponent.SetMaterial` (`self.Bulb`) 0 "/Game/Workplace/Materials/M_Glow_Green.M_Glow_Green")
                      (bind _asbp_button_3 (cast `/Game/Workplace/Blueprints/BP_Button` (`ChildActorComponent.ChildActor` (`self.Button`))))
                      (set `/Game/Workplace/Blueprints/BP_Button.State` false _asbp_button_3)
                      (set `/Game/Workplace/Blueprints/BP_Button.PreState` false _asbp_button_3)
                      (set `self.Broke` false)
                      (set `self.Print` false)
                      (set `self.ThisPrinterUsed` false)))
                  (else
                    (set `/Game/Workplace/Blueprints/GlobalVariables.ManipulatorBusy` true _asglobal_variables_5)
                    (set `self.ThisPrinterUsed` true)
                    (bind _outactors (`GameplayStatics.GetAllActorsWithInterface` "/Game/Workplace/Blueprints/BI_manipulator_Take.BI_manipulator_Take_C"))
                    (message `/Game/Workplace/Blueprints/BI_manipulator_Take.Take` _outactors (`KismetSystemLibrary.GetDisplayName` self) (`self.SDIndex`) _asmaterial (`SceneComponent.K2_GetComponentScale` (`self.PrintedObject`)))))))
            (else
              (`PrimitiveComponent.SetMaterial` (`self.Bulb`) 0 "/Game/Workplace/Materials/M_Glow_Red.M_Glow_Red")
              (bind _asbp_button_4 (cast `/Game/Workplace/Blueprints/BP_Button` (`ChildActorComponent.ChildActor` (`self.Button`))))
              (set `/Game/Workplace/Blueprints/BP_Button.State` true _asbp_button_4)
              (set `/Game/Workplace/Blueprints/BP_Button.PreState` true _asbp_button_4)))
          (elif (`self.SpoolAdded`)
            ;[1 1 1] Проверка наличия SD
            (`PrimitiveComponent.SetMaterial` (`self.Bulb`) 0 "/Game/Workplace/Materials/M_Glow_Green.M_Glow_Green")
            (bind _asglobal_variables_7 (cast `/Game/Workplace/Blueprints/GlobalVariables` (`GameplayStatics.GetGameInstance`)))
            (if (`/Game/Workplace/Blueprints/GlobalVariables.SDAvailable` _asglobal_variables_7)
              (if (`/Game/Workplace/Blueprints/GlobalVariables.SDWritten` _asglobal_variables_7)
                ;[1 1 1] Проверка на нажатие кнопки
                (bind _asbp_button_5 (cast `/Game/Workplace/Blueprints/BP_Button` (`ChildActorComponent.ChildActor` (`self.Button`))))
                (if (`/Game/Workplace/Blueprints/BP_Button.State` _asbp_button_5)
                  ;[1 1 1] Сохранение параметров печати
                  (bind _asglobal_variables_8 (cast `/Game/Workplace/Blueprints/GlobalVariables` (`GameplayStatics.GetGameInstance`)))
                  (set `self.SDIndex` (`/Game/Workplace/Blueprints/GlobalVariables.SDIndex` _asglobal_variables_8))
                  (set `self.SDFilling` (`/Game/Workplace/Blueprints/GlobalVariables.SDFilling` _asglobal_variables_8))
                  (set `self.SDSupport` (`/Game/Workplace/Blueprints/GlobalVariables.SDSupport` _asglobal_variables_8))
                  (set `/Game/Workplace/Blueprints/GlobalVariables.SDWritten` false _asglobal_variables_8)
                  ;[1 1 1] Настройки длительности печати
                  (set `self.Print` true)
                  (if (`self.SDSupport`)
                    (bind _y (`self.ScaleTransform` (`KismetMathLibrary.Conv_IntToDouble` (- 100 (`self.SDFilling`))) 0.0 100.0 1.0 (/ (`self.MaxSpeed`) 2.0)))
                    (bind _asabp_3d_printer_up_4 (cast `/Game/Workplace/Animations/ABP_3D_Printer_UP` (`SkeletalMeshComponent.GetAnimInstance` (`self.Printer`))))
                    (bind _output_get (set `/Game/Workplace/Animations/ABP_3D_Printer_UP.Speed` _y _asabp_3d_printer_up_4))
                    (set `/Game/Workplace/Animations/ABP_3D_Printer_UP.Phase1` true _asabp_3d_printer_up_4)
                    (bind _y_2 (`self.ScaleTransform` _output_get 1.0 (/ (`self.MaxSpeed`) 2.0) 0.1 0.3))
                    (set `self.Broke` (`KismetMathLibrary.RandomBoolWithWeight` _y_2))
                    (set `self.ThisPrinterUsed` false)
                    (else
                      (bind _y_3 (`self.ScaleTransform` (`KismetMathLibrary.Conv_IntToDouble` (- 100 (`self.SDFilling`))) 0.0 100.0 (/ _maxspeed_2 2.0) _maxspeed_2))
                      (bind _asabp_3d_printer_up_5 (cast `/Game/Workplace/Animations/ABP_3D_Printer_UP` (`SkeletalMeshComponent.GetAnimInstance` (`self.Printer`))))
                      (bind _output_get_2 (set `/Game/Workplace/Animations/ABP_3D_Printer_UP.Speed` _y_3 _asabp_3d_printer_up_5))
                      (set `/Game/Workplace/Animations/ABP_3D_Printer_UP.Phase1` true _asabp_3d_printer_up_5)
                      (bind _y_4 (`self.ScaleTransform` _output_get_2 (/ _maxspeed 2.0) _maxspeed 0.3 0.8))
                      (set `self.Broke` (`KismetMathLibrary.RandomBoolWithWeight` _y_4))
                      (set `self.ThisPrinterUsed` false))))
                (else
                  ;[1 1 1] Нет SD
                  (bind _asbp_button_6 (cast `/Game/Workplace/Blueprints/BP_Button` (`ChildActorComponent.ChildActor` (`self.Button`)) :!label _label))
                  (set `/Game/Workplace/Blueprints/BP_Button.State` false _asbp_button_6)
                  (set `/Game/Workplace/Blueprints/BP_Button.PreState` false _asbp_button_6)))
              (else
                (goto _label)))
            (else
              ;[1 1 1] нет бобины
              (`PrimitiveComponent.SetMaterial` (`self.Bulb`) 0 "/Game/Workplace/Materials/M_Glow_Red.M_Glow_Red")
              (bind _asbp_button_7 (cast `/Game/Workplace/Blueprints/BP_Button` (`ChildActorComponent.ChildActor` (`self.Button`))))
              (set `/Game/Workplace/Blueprints/BP_Button.State` false _asbp_button_7)
              (set `/Game/Workplace/Blueprints/BP_Button.PreState` false _asbp_button_7))))
        (else
          ;[1 1 1] Не началась нужная фааза
          (`PrimitiveComponent.SetMaterial` (`self.Bulb`) 0 "/Game/FirstPerson/Meshes/BaseMaterial.BaseMaterial")
          (bind _asbp_button_8 (cast `/Game/Workplace/Blueprints/BP_Button` (`ChildActorComponent.ChildActor` (`self.Button`))))
          (set `/Game/Workplace/Blueprints/BP_Button.State` false _asbp_button_8)
          (set `/Game/Workplace/Blueprints/BP_Button.PreState` false _asbp_button_8))))))

(fn `ChangeBlueSpool`
  (params (ActorReference :type "Actor Object Reference"))
  (bind _asbp_spool_blue (cast `/Game/Workplace/Blueprints/BP_Spool_Blue` ActorReference))
  (`PrimitiveComponent.SetMaterial` (`self.Bulb`) 0 "/Game/Workplace/Materials/M_Glow_Green.M_Glow_Green")
  (bind _asbp_empty_spool (cast `/Game/Workplace/Blueprints/BP_Empty_Spool` (`ChildActorComponent.ChildActor` (`self.Spool`))))
  ;[1 1 1] Спавним бобину
  (if (`/Game/Workplace/Blueprints/BP_Empty_Spool.Colored` _asbp_empty_spool)
    (`|SpawnActorFromClass` (`GameplayStatics.GetObjectClass` (`self.Class`)) (`KismetMathLibrary.MakeTransform` (`SceneComponent.K2_GetComponentLocation` (`self.DropPoint`)) (struct) (`KismetMathLibrary.Conv_DoubleToVector` (`self.Scale`))) "Undefined" "OverrideRootScale" null null))
  ;[1 1 1] Задаем цвет
  (set `self.Class` _asbp_spool_blue)
  (set `/Game/Workplace/Blueprints/BP_Empty_Spool.Colored` true _asbp_empty_spool)
  (bind _asmaterial (cast `Material` (`PrimitiveComponent.GetMaterial` (`/Game/Workplace/Blueprints/BP_Spool_Blue.Plastic` _asbp_spool_blue) 0)))
  (set `/Game/Workplace/Blueprints/BP_Empty_Spool.Material` _asmaterial _asbp_empty_spool)
  (`self.K2_DestroyActor` _asbp_spool_blue))

(fn `ChangeGreenSpool`
  (params (ActorReference :type "Actor Object Reference"))
  (bind _asbp_spool_green (cast `/Game/Workplace/Blueprints/BP_Spool_Green` ActorReference))
  (`PrimitiveComponent.SetMaterial` (`self.Bulb`) 0 "/Game/Workplace/Materials/M_Glow_Green.M_Glow_Green")
  (bind _asbp_empty_spool (cast `/Game/Workplace/Blueprints/BP_Empty_Spool` (`ChildActorComponent.ChildActor` (`self.Spool`))))
  ;[1 1 1] Спавним бобину
  (if (`/Game/Workplace/Blueprints/BP_Empty_Spool.Colored` _asbp_empty_spool)
    (`|SpawnActorFromClass` (`GameplayStatics.GetObjectClass` (`self.Class`)) (`KismetMathLibrary.MakeTransform` (`SceneComponent.K2_GetComponentLocation` (`self.DropPoint`)) (struct) (`KismetMathLibrary.Conv_DoubleToVector` (`self.Scale`))) "Undefined" "OverrideRootScale" null null))
  ;[1 1 1] Задаем цвет
  (set `self.Class` _asbp_spool_green)
  (set `/Game/Workplace/Blueprints/BP_Empty_Spool.Colored` true _asbp_empty_spool)
  (bind _asmaterial (cast `Material` (`PrimitiveComponent.GetMaterial` (`/Game/Workplace/Blueprints/BP_Spool_Green.Plastic` _asbp_spool_green) 0)))
  (set `/Game/Workplace/Blueprints/BP_Empty_Spool.Material` _asmaterial _asbp_empty_spool)
  (`self.K2_DestroyActor` _asbp_spool_green))

(fn `ChangeRedSpool`
  (params (ActorReference :type "Actor Object Reference"))
  (bind _asbp_spool_red (cast `/Game/Workplace/Blueprints/BP_Spool_Red` ActorReference))
  (`PrimitiveComponent.SetMaterial` (`self.Bulb`) 0 "/Game/Workplace/Materials/M_Glow_Green.M_Glow_Green")
  (bind _asbp_empty_spool (cast `/Game/Workplace/Blueprints/BP_Empty_Spool` (`ChildActorComponent.ChildActor` (`self.Spool`))))
  ;[1 1 1] Спавним бобину
  (if (`/Game/Workplace/Blueprints/BP_Empty_Spool.Colored` _asbp_empty_spool)
    (`|SpawnActorFromClass` (`GameplayStatics.GetObjectClass` (`self.Class`)) (`KismetMathLibrary.MakeTransform` (`SceneComponent.K2_GetComponentLocation` (`self.DropPoint`)) (struct) (`KismetMathLibrary.Conv_DoubleToVector` (`self.Scale`))) "Undefined" "OverrideRootScale" null null))
  ;[1 1 1] Задаем цвет
  (set `self.Class` _asbp_spool_red)
  (set `/Game/Workplace/Blueprints/BP_Empty_Spool.Colored` true _asbp_empty_spool)
  (bind _asmaterial (cast `Material` (`PrimitiveComponent.GetMaterial` (`/Game/Workplace/Blueprints/BP_Spool_Red.Plastic` _asbp_spool_red) 0)))
  (set `/Game/Workplace/Blueprints/BP_Empty_Spool.Material` _asmaterial _asbp_empty_spool)
  (`self.K2_DestroyActor` _asbp_spool_red))

(fn `ChangeYellowSpool`
  (params (ActorReference :type "Actor Object Reference"))
  (bind _asbp_spool_yellow (cast `/Game/Workplace/Blueprints/BP_Spool_Yellow` ActorReference))
  (`PrimitiveComponent.SetMaterial` (`self.Bulb`) 0 "/Game/Workplace/Materials/M_Glow_Green.M_Glow_Green")
  (bind _asbp_empty_spool (cast `/Game/Workplace/Blueprints/BP_Empty_Spool` (`ChildActorComponent.ChildActor` (`self.Spool`))))
  ;[1 1 1] Спавним бобину
  (if (`/Game/Workplace/Blueprints/BP_Empty_Spool.Colored` _asbp_empty_spool)
    (`|SpawnActorFromClass` (`GameplayStatics.GetObjectClass` (`self.Class`)) (`KismetMathLibrary.MakeTransform` (`SceneComponent.K2_GetComponentLocation` (`self.DropPoint`)) (struct) (`KismetMathLibrary.Conv_DoubleToVector` (`self.Scale`))) "Undefined" "OverrideRootScale" null null))
  ;[1 1 1] Задаем цвет
  (set `self.Class` _asbp_spool_yellow)
  (set `/Game/Workplace/Blueprints/BP_Empty_Spool.Colored` true _asbp_empty_spool)
  (bind _asmaterial (cast `Material` (`PrimitiveComponent.GetMaterial` (`/Game/Workplace/Blueprints/BP_Spool_Yellow.plastic` _asbp_spool_yellow) 0)))
  (set `/Game/Workplace/Blueprints/BP_Empty_Spool.Material` _asmaterial _asbp_empty_spool)
  (`self.K2_DestroyActor` _asbp_spool_yellow))

(fn `ScaleTransform`
  (params (X :type "Float (double-precision)") (XMin1 :type "Float (double-precision)") (XMax1 :type "Float (double-precision)") (XMin2 :type "Float (double-precision)") (XMax2 :type "Float (double-precision)"))
  (returns (Y :type "Float (double-precision)"))
  (return (+ (/ (* (- X XMin1) (- XMax2 XMin2)) (- XMax1 XMin1)) XMin2)))

(fn `UserConstructionScript`)