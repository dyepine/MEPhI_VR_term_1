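; BP_TransferObject is a moving object that travels to either the table or a stamping machine, based on its type in GlobalVariables.
; StartTransfering uses timelines to interpolate its position between stored points.
; Type 0 objects travel straight to the end, increment the ready count and notify BI_AddObjectsOnTable actors.
; Other types turn off upon passing the trigger distance, then notify BI_AddObjectsOnMachine actors; both routes destroy the object on arrival.
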(event `/Game/Workplace/Blueprints/BI_StartTransfering.StartTransfering`
  ;[1 1 1] Готовый обьект или обрабатывается?
  (bind _asglobal_variables (cast `/Game/Workplace/Blueprints/GlobalVariables` (`GameplayStatics.GetGameInstance`)))
  (if (== (`|GetArrayItem` (`/Game/Workplace/Blueprints/GlobalVariables.TypeTrackObjects` _asglobal_variables) (`self.ObjectNumber`)) 0)
    ;[1 1 1] Движение готовых обьектов до стола
    (bind (_direction _transfering) (`Timeline|Transfering=0` :!via `PlayFromStart`)
      (:`Update`
        (`self.K2_SetActorLocation` (+ (`self.StartPositionVariable`) (* (- (`self.EndPositionVariable`) (`self.StartPositionVariable`)) _transfering))))
      (:`Finished`
        ;[1 1 1] Что делать при достижении конца
        (`self.K2_DestroyActor`)
        (bind _outactors (`GameplayStatics.GetAllActorsWithInterface` "/Game/Workplace/Blueprints/BI_AddObjectsOnTable.BI_AddObjectsOnTable_C"))
        (bind _asglobal_variables_2 (cast `/Game/Workplace/Blueprints/GlobalVariables` (`GameplayStatics.GetGameInstance`)))
        (set `/Game/Workplace/Blueprints/GlobalVariables.NumReadyTrackObjects` (+ (`/Game/Workplace/Blueprints/GlobalVariables.NumReadyTrackObjects` _asglobal_variables_2) 1) _asglobal_variables_2)
        (message `/Game/Workplace/Blueprints/BI_AddObjectsOnTable.AddObjectsOnTable` _outactors (`self.ObjectNumber`))))
    (else
      ;[1 1 1] Движение до триггера
      (bind (_direction_2 _transfering_2) (`Timeline|Transfering>0` :!via `PlayFromStart` :!label _label)
        (:`Update`
          (`self.K2_SetActorLocation` (+ (* (- (`self.EndPositionVariable`) (`self.StartPositionVariable`)) _transfering_2) (`self.StartPositionVariable`)))
          (if (> (* _transfering_2 (`KismetMathLibrary.VSize` (- (`self.EndPositionVariable`) (`self.StartPositionVariable`)))) (`KismetMathLibrary.VSize` (- (`self.StartTriggerVariable`) (`self.StartPositionVariable`))))
            (`|ExecutionSequence`
              (:`then_0`
                (goto _label :!via `Stop`))
              (:`then_1`
                ;[1 1 1] Движение обьекта до штампа
                (bind (_direction_3 _transfer_to_processing) (`Timeline|Transfering=trigger` :!via `PlayFromStart`)
                  (:`Update`
                    (`self.K2_SetActorLocation` (+ (`self.StartTriggerVariable`) (* (- (`self.EndTriggerVariable`) (`self.StartTriggerVariable`)) _transfer_to_processing))))
                  (:`Finished`
                    ;[1 1 1] Что делать с обьектом при достижении штампа
                    (`self.K2_DestroyActor`)
                    (bind _outactors_2 (`GameplayStatics.GetAllActorsWithInterface` "/Game/Workplace/Blueprints/BI_AddObjectsOnMachine.BI_AddObjectsOnMachine_C"))
                    (message `/Game/Workplace/Blueprints/BI_AddObjectsOnMachine.AddObjectsOnMachine` _outactors_2 (`self.ObjectNumber`))))))))))))

(fn `UserConstructionScript`)