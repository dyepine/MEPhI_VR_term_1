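; BP_ObjectsGiver is a dispenser actor that spawns a physics object chosen by index.
; Its Issue event spawns a BP_GivenObjects at the Sphere component's location, using per-index rotation and scale arrays from the GlobalVariables game instance.
; It then passes the index to the new actor, assigns the matching SDObjects mesh and enables physics simulation as a PhysicsBody.
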(event `/Game/Workplace/Blueprints/BI_Issue.Issue`
  (params (Index :type Integer))
  (set `self.Index` Index)
  (bind _asglobal_variables (cast `/Game/Workplace/Blueprints/GlobalVariables` (`GameplayStatics.GetGameInstance`)))
  (bind _returnvalue (`|SpawnActorFromClass` "/Game/Workplace/Blueprints/BP_GivenObjects.BP_GivenObjects_C" (`KismetMathLibrary.MakeTransform` (`SceneComponent.K2_GetComponentLocation` (`self.Sphere`)) (`KismetMathLibrary.Conv_VectorToRotator` (`|GetArrayItem` (`/Game/Workplace/Blueprints/GlobalVariables.SDObjectsRotation` _asglobal_variables) (`self.Index`))) (`KismetMathLibrary.Conv_DoubleToVector` (`|GetArrayItem` (`/Game/Workplace/Blueprints/GlobalVariables.SDObjectsScale` _asglobal_variables) (`self.Index`)))) "Undefined" "OverrideRootScale" null null))
  (set `/Game/Workplace/Blueprints/BP_GivenObjects.Index` (`self.Index`) _returnvalue)
  (bind _asglobal_variables_2 (cast `/Game/Workplace/Blueprints/GlobalVariables` (`GameplayStatics.GetGameInstance`)))
  (bind _givenobject (`/Game/Workplace/Blueprints/BP_GivenObjects.GivenObject` _returnvalue))
  (`StaticMeshComponent.SetStaticMesh` _givenobject (`|GetArrayItem` (`/Game/Workplace/Blueprints/GlobalVariables.SDObjects` _asglobal_variables_2) (`self.Index`)))
  (`PrimitiveComponent.SetSimulatePhysics` _givenobject true)
  (`PrimitiveComponent.SetCollisionObjectType` _givenobject "ECC_PhysicsBody"))

(fn `UserConstructionScript`)