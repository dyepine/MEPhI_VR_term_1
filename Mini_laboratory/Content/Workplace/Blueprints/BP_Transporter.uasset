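; BP_Transporter is a track spawner that feeds transfer objects onto a route defined by start, end and two trigger marker components.
; BeginPlay caches the marker positions.
; Tick polls the AddObject flag in the GlobalVariables game instance, then after a delay clears it and spawns a BP_TransferObject until NumTrackObjects is reached.
; Each spawn gets its indexed mesh, scale and route positions before StartTransferingMessage starts it.
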(event `self.ReceiveBeginPlay`
  ;[1 1 1] Задание начальных переменных
  (set `self.StartPositionVariable` (`SceneComponent.K2_GetComponentLocation` (`self.StartPosition`)))
  (set `self.EndPositionVector` (`SceneComponent.K2_GetComponentLocation` (`self.EndPosition`)))
  (set `self.StartTriggerPositionVector` (`SceneComponent.K2_GetComponentLocation` (`self.StartTriggerPosition`)))
  (set `self.EndTriggerPositionVector` (`SceneComponent.K2_GetComponentLocation` (`self.EndTriggerPosition`)))
  (set `self.ObjectNumber` 0))

(event `self.ReceiveTick`
  (params (DeltaSeconds :type "Float (single-precision)"))
  ;[1 1 1] Создание обьекта на трассе по команде addobject
  (bind _asglobal_variables (cast `/Game/Workplace/Blueprints/GlobalVariables` (`GameplayStatics.GetGameInstance`)))
  (if (`/Game/Workplace/Blueprints/GlobalVariables.AddObject` _asglobal_variables)
    (`KismetSystemLibrary.Delay` (`self.delay`))
    (bind _asglobal_variables_2 (cast `/Game/Workplace/Blueprints/GlobalVariables` (`GameplayStatics.GetGameInstance`)))
    (set `/Game/Workplace/Blueprints/GlobalVariables.AddObject` false _asglobal_variables_2)
    (if (< (`self.ObjectNumber`) (`/Game/Workplace/Blueprints/GlobalVariables.NumTrackObjects` _asglobal_variables_2))
      (bind _returnvalue (`|SpawnActorFromClass` "/Game/Workplace/Blueprints/BP_TransferObject.BP_TransferObject_C" (`KismetMathLibrary.MakeTransform` (`self.StartPositionVariable`)) "Undefined" "OverrideRootScale" null null))
      ;[1 1 1] Задание переменных созданного обьекта
      (bind _asglobal_variables_3 (cast `/Game/Workplace/Blueprints/GlobalVariables` (`GameplayStatics.GetGameInstance`)))
      (bind _transferedobject (`/Game/Workplace/Blueprints/BP_TransferObject.TransferedObject` _returnvalue))
      (`StaticMeshComponent.SetStaticMesh` _transferedobject (`|GetArrayItem` (`/Game/Workplace/Blueprints/GlobalVariables.TrackObjects` _asglobal_variables_3) (`self.ObjectNumber`)))
      (bind _asglobal_variables_4 (cast `/Game/Workplace/Blueprints/GlobalVariables` (`GameplayStatics.GetGameInstance`)))
      (`SceneComponent.SetWorldScale3D` _transferedobject (`KismetMathLibrary.Conv_DoubleToVector` (`|GetArrayItem` (`/Game/Workplace/Blueprints/GlobalVariables.ScaleTrackObjects` _asglobal_variables_4) (`self.ObjectNumber`))))
      (set `/Game/Workplace/Blueprints/BP_TransferObject.ObjectNumber` (`self.ObjectNumber`) _returnvalue)
      (set `/Game/Workplace/Blueprints/BP_TransferObject.StartTriggerVariable` (`self.StartTriggerPositionVector`) _returnvalue)
      (set `/Game/Workplace/Blueprints/BP_TransferObject.EndTriggerVariable` (`self.EndTriggerPositionVector`) _returnvalue)
      (set `/Game/Workplace/Blueprints/BP_TransferObject.StartPositionVariable` (`self.StartPositionVariable`) _returnvalue)
      (set `/Game/Workplace/Blueprints/BP_TransferObject.EndPositionVariable` (`self.EndPositionVector`) _returnvalue)
      (set `self.ObjectNumber` (+ (`self.ObjectNumber`) 1))
      (message `/Game/Workplace/Blueprints/BPI_StartTransfering.StartTransfering` _returnvalue))))

(fn `UserConstructionScript`)