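; Workplace rail that carries a child BP_Manipulator to one of two 3D printers to pick up a printed object and back to drop it in a box.
; Take picks the printer by name, and chained timelines slide the arm linearly from start through a bend point to that printer.
; SetObject copies mesh and rotation from GlobalVariables, plus the passed material and scale, onto the held object.
; MoveBack retraces the path, then sends the manipulator Drop.
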(event `self.ReceiveBeginPlay`
  ;[1 1 1] Телепортируем руку в начальную точку
  (`SceneComponent.K2_SetWorldLocation` (`self.Manipulator`) (`SceneComponent.K2_GetComponentLocation` (`self.StartPoint`)) false true)
  (set `self.SDIndex` 0)
  (set `self.Material` null)
  (set `self.Scale` (0.0 0.0 0.0))
  (set `self.EndPosition` (0.0 0.0 0.0)))

(event `/Game/Workplace/Blueprints/BI_manipulator_Take.Take`
  (params (PrinterName :type String) (SDIndex :type Integer) (Material :type "Material Object Reference") (Scale :type "Vector Structure"))
  (bind _returnvalue (`SceneComponent.K2_GetComponentLocation` (`self.StartPoint`)))
  (bind _returnvalue_2 (`SceneComponent.K2_GetComponentLocation` (`self.BendPoint`)))
  (bind _returnvalue_3 (`SceneComponent.K2_GetComponentLocation` (`self.BendPoint`)))
  (set `self.Material` Material)
  (set `self.SDIndex` SDIndex)
  (set `self.Scale` Scale)
  ;[1 1 1] Начало движения манипулятора
  (bind (_direction _func) (`Timeline|StartMove` :!via `PlayFromStart`)
    (:`Update`
      (`SceneComponent.K2_SetWorldLocation` (`self.Manipulator`) (+ (* (- (`SceneComponent.K2_GetComponentLocation` (`self.BendPoint`)) _returnvalue) _func) _returnvalue) false true))
    (:`Finished`
      (if (`KismetStringLibrary.EqualEqual_StrStr` PrinterName "BP_3D_Printer_UP")
        ;[1 1 1] Захват объекта из 1 принтера
        (bind (_direction_2 _func_2) (`Timeline|FirstPrinter` :!via `PlayFromStart`)
          (:`Update`
            (`SceneComponent.K2_SetWorldLocation` (`self.Manipulator`) (+ (* (- (`SceneComponent.K2_GetComponentLocation` (`self.PrinterPoint1`)) _returnvalue_2) _func_2) _returnvalue_2) false true))
          (:`Finished`
            (`self.SetObject`)
            (message `/Game/Workplace/Blueprints/BI_Manipulator.Mode` (`ChildActorComponent.ChildActor` (`self.Manipulator`)) "Take" 0 null)))
        (else
          ;[1 1 1] Захват объекта из 1 принтера
          (bind (_direction_3 _func_3) (`Timeline|SecondPrinter` :!via `PlayFromStart`)
            (:`Update`
              (`SceneComponent.K2_SetWorldLocation` (`self.Manipulator`) (+ (* (- (`SceneComponent.K2_GetComponentLocation` (`self.PrinterPoint2`)) _returnvalue_3) _func_3) _returnvalue_3) false true))
            (:`Finished`
              (`self.SetObject`)
              (message `/Game/Workplace/Blueprints/BI_Manipulator.Mode` (`ChildActorComponent.ChildActor` (`self.Manipulator`)) "Take" 0 null))))))))

(event `/Game/Workplace/Blueprints/BI_MoveBack.MoveBack`
  (bind _endposition (`self.EndPosition`))
  (bind _returnvalue (`SceneComponent.K2_GetComponentLocation` (`self.BendPoint`)))
  ;[1 1 1] Поехать назад для сброса в коробку
  (set `self.EndPosition` (`SceneComponent.K2_GetComponentLocation` (`self.Manipulator`)))
  (bind (_direction _func) (`Timeline|MoveBack1` :!via `PlayFromStart`)
    (:`Update`
      (`SceneComponent.K2_SetWorldLocation` (`self.Manipulator`) (+ (* (- (`SceneComponent.K2_GetComponentLocation` (`self.BendPoint`)) _endposition) _func) _endposition) false true))
    (:`Finished`
      (bind (_direction_2 _func_2) (`Timeline|MoveBack2` :!via `PlayFromStart`)
        (:`Update`
          (`SceneComponent.K2_SetWorldLocation` (`self.Manipulator`) (+ (* (- (`SceneComponent.K2_GetComponentLocation` (`self.StartPoint`)) _returnvalue) _func_2) _returnvalue) false true))
        (:`Finished`
          (message `/Game/Workplace/Blueprints/BI_Manipulator.Mode` (`ChildActorComponent.ChildActor` (`self.Manipulator`)) "Drop" (`self.SDIndex`) (`self.Material`)))))))

(fn `SetObject`
  (bind _asbp_manipulator (cast `/Game/Workplace/Blueprints/BP_Manipulator` (`ChildActorComponent.ChildActor` (`self.Manipulator`))))
  (bind _asglobal_variables (cast `/Game/Workplace/Blueprints/GlobalVariables` (`GameplayStatics.GetGameInstance`)))
  (bind _object (`/Game/Workplace/Blueprints/BP_Manipulator.Object` _asbp_manipulator))
  (`StaticMeshComponent.SetStaticMesh` _object (`|GetArrayItem` (`/Game/Workplace/Blueprints/GlobalVariables.SDObjects` _asglobal_variables) (`self.SDIndex`)))
  (`PrimitiveComponent.SetMaterial` _object 0 (`self.Material`))
  (bind _asglobal_variables_2 (cast `/Game/Workplace/Blueprints/GlobalVariables` (`GameplayStatics.GetGameInstance`)))
  (`SceneComponent.K2_SetWorldRotation` _object (`KismetMathLibrary.Conv_VectorToRotator` (`|GetArrayItem` (`/Game/Workplace/Blueprints/GlobalVariables.SDObjectsRotation` _asglobal_variables_2) (`self.SDIndex`))) false false)
  (`SceneComponent.SetWorldScale3D` _object (`self.Scale`))
  (bind _asbp_manipulator_2 (cast `/Game/Workplace/Blueprints/BP_Manipulator` (`ChildActorComponent.ChildActor` (`self.Manipulator`))))
  (`SceneComponent.K2_AttachToComponent` (`/Game/Workplace/Blueprints/BP_Manipulator.Object` _asbp_manipulator_2) (`/Game/Workplace/Blueprints/BP_Manipulator.Manipulator` _asbp_manipulator_2) "Object" "KeepRelative" "KeepRelative" "KeepWorld" true))

(fn `StartMovement`)

(fn `UserConstructionScript`)