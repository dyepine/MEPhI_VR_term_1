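; 3D printer actor in the workplace that turns a start-button press into a request to add an object, via the GameInstance's AddObject flag.
; StartPrint consumes a Permission gate, waits a delay, then resets the button and sets the flag; AddObjectsonTable re-arms it in phase 1.
; After the first print, Tick polls the GameInstance's hit button by display name, repeating prints in phase 1 and only resetting the button in phase 2.
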(event `self.ReceiveBeginPlay`
  (set `self.Permission` true)
  (set `self.FirstPermission` false))

(event `/Game/Workplace/Blueprints/BPI_StartPrint.StartPrint`
  (params (HitResult :type "Actor Object Reference"))
  (set `self.Button` HitResult)
  (if (`self.Permission`)
    (set `self.Permission` false)
    (`KismetSystemLibrary.Delay` (`self.delay`))
    (bind _asbp_button (cast `/Game/Workplace/Blueprints/BP_Button` (`self.Button`)))
    (set `/Game/Workplace/Blueprints/BP_Button.PreState` false _asbp_button)
    (set `/Game/Workplace/Blueprints/BP_Button.State` false _asbp_button)
    (bind _asglobal_variables (cast `/Game/Workplace/Blueprints/GlobalVariables` (`GameplayStatics.GetGameInstance`)))
    (set `/Game/Workplace/Blueprints/GlobalVariables.AddObject` true _asglobal_variables)
    (set `self.FirstPermission` true)))

(event `/Game/Workplace/Blueprints/BPI_AddObjectsOnTable.AddObjectsOnTable`
  (params (NumObject :type Integer))
  (bind _asglobal_variables (cast `/Game/Workplace/Blueprints/GlobalVariables` (`GameplayStatics.GetGameInstance`)))
  (if (== (`/Game/Workplace/Blueprints/GlobalVariables.LevelPhase` _asglobal_variables) 1)
    (if (not (`self.Permission`))
      (set `self.Permission` true))))

(event `self.ReceiveTick`
  (params (DeltaSeconds :type "Float (single-precision)"))
  (if (`self.FirstPermission`)
    (`|ExecutionSequence`
      (:`then_0`
        (bind _asglobal_variables (cast `/Game/Workplace/Blueprints/GlobalVariables` (`GameplayStatics.GetGameInstance`)))
        (if (== (`/Game/Workplace/Blueprints/GlobalVariables.LevelPhase` _asglobal_variables) 1)
          (bind _asglobal_variables_2 (cast `/Game/Workplace/Blueprints/GlobalVariables` (`GameplayStatics.GetGameInstance`)))
          (bind _asbp_button (cast `/Game/Workplace/Blueprints/BP_Button` (`/Game/Workplace/Blueprints/GlobalVariables.HitResult` _asglobal_variables_2)))
          (if (`KismetStringLibrary.EqualEqual_StrStr` (`KismetSystemLibrary.GetDisplayName` _asbp_button) "StartPrint_Button")
            (if (`/Game/Workplace/Blueprints/BP_Button.State` _asbp_button)
              (if (`/Game/Workplace/Blueprints/BP_Button.PreState` _asbp_button)
                (if (`self.Permission`)
                  (`KismetSystemLibrary.Delay` (`self.delay`))
                  (set `self.Permission` false)
                  (bind _asbp_button_2 (cast `/Game/Workplace/Blueprints/BP_Button` (`self.Button`)))
                  (set `/Game/Workplace/Blueprints/BP_Button.PreState` false _asbp_button_2)
                  (set `/Game/Workplace/Blueprints/BP_Button.State` false _asbp_button_2)
                  (bind _asglobal_variables_3 (cast `/Game/Workplace/Blueprints/GlobalVariables` (`GameplayStatics.GetGameInstance`)))
                  (set `/Game/Workplace/Blueprints/GlobalVariables.AddObject` true _asglobal_variables_3)
                  (else
                    (bind _asbp_button_3 (cast `/Game/Workplace/Blueprints/BP_Button` (`self.Button`)))
                    (set `/Game/Workplace/Blueprints/BP_Button.PreState` false _asbp_button_3)
                    (set `/Game/Workplace/Blueprints/BP_Button.State` false _asbp_button_3))))))))
      (:`then_1`
        (bind _asglobal_variables_4 (cast `/Game/Workplace/Blueprints/GlobalVariables` (`GameplayStatics.GetGameInstance`)))
        (if (== (`/Game/Workplace/Blueprints/GlobalVariables.LevelPhase` _asglobal_variables_4) 2)
          (bind _asglobal_variables_5 (cast `/Game/Workplace/Blueprints/GlobalVariables` (`GameplayStatics.GetGameInstance`)))
          (bind _asbp_button_4 (cast `/Game/Workplace/Blueprints/BP_Button` (`/Game/Workplace/Blueprints/GlobalVariables.HitResult` _asglobal_variables_5)))
          (if (`KismetStringLibrary.EqualEqual_StrStr` (`KismetSystemLibrary.GetDisplayName` _asbp_button_4) "StartPrint_Button")
            (if (`/Game/Workplace/Blueprints/BP_Button.State` _asbp_button_4)
              (if (`/Game/Workplace/Blueprints/BP_Button.PreState` _asbp_button_4)
                (bind _asbp_button_5 (cast `/Game/Workplace/Blueprints/BP_Button` (`self.Button`)))
                (set `/Game/Workplace/Blueprints/BP_Button.PreState` false _asbp_button_5)
                (set `/Game/Workplace/Blueprints/BP_Button.State` false _asbp_button_5)))))))))

(fn `UserConstructionScript`)