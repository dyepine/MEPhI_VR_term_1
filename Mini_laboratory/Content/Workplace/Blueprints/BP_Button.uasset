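; BP_Button is a clickable toggle button that displays its boolean State by swapping the Button component's material from a Materials array.
; Tick polls the GlobalVariables game instance: while this actor is the HitResult and left mouse is pressed, PreState flips opposite State.
; When the mouse is no longer pressed, State takes PreState's value, so each click toggles once.
; A touch-begin event resets both flags to false.
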(event `self.ReceiveActorOnInputTouchBegin`
  (params (FingerIndex :type "ETouchIndex Enum" :default "Touch1"))
  ;[1 1 1] Установить начальные переменные
  (set `self.State` false)
  (set `self.PreState` false))

(event `self.ReceiveTick`
  (params (DeltaSeconds :type "Float (single-precision)"))
  ;[1 1 1] Event Tick
  (`|ExecutionSequence`
    (:`then_0`
      ;[1 1 1] Задает материал
      (`PrimitiveComponent.SetMaterial` (`self.Button`) 0 (`|GetArrayItem` (`self.Materials`) (`KismetMathLibrary.Conv_BoolToInt` (`self.State`)))))
    (:`then_1`
      ;[1 1 1] Переключение режимов кнопки
      (bind _asglobal_variables (cast `/Game/Workplace/Blueprints/GlobalVariables` (`GameplayStatics.GetGameInstance`)))
      (if (== self (`/Game/Workplace/Blueprints/GlobalVariables.HitResult` _asglobal_variables))
        (if (`/Game/Workplace/Blueprints/GlobalVariables.LeftMousePressed` _asglobal_variables)
          (if (`self.State`)
            (if (`self.PreState`)
              (set `self.PreState` false))
            (elif (not (`self.PreState`))
              (set `self.PreState` true))))))
    (:`then_2`
      (bind _asglobal_variables_2 (cast `/Game/Workplace/Blueprints/GlobalVariables` (`GameplayStatics.GetGameInstance`)))
      (if (`/Game/Workplace/Blueprints/GlobalVariables.LeftMousePressed` _asglobal_variables_2)
        _
        (elif (`self.State`)
          (if (not (`self.PreState`))
            (set `self.State` false))
          (elif (`self.PreState`)
            (set `self.State` true)))))))

(fn `UserConstructionScript`)