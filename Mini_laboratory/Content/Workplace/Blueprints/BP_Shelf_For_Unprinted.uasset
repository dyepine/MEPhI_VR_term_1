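; Shelf that stocks the workplace with unprinted parts (arms, directions, lidar, motors) once the global LevelPhase reaches 4.
; BeginPlay sums box counts of non-printed objects from GlobalVariables to compute even spacing between StartPoint and EndPoint.
; Tick polls the phase and, behind a one-shot flag, spawns a hardcoded set of physics-simulated BP_Shelf_Objects.
; Each takes its mesh, rotation and scale from GlobalVariables and the next slot from GetPoint.
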(event `self.ReceiveBeginPlay`
  ;[1 1 1] Задаем начальные условия
  (set `self.LevelPhaseIsBiggerThan4` false)
  (`self.Counter`)
  (set `self.NumberOfObject` 0)
  (set `self.Step` (/ (- (`SceneComponent.K2_GetComponentLocation` (`self.EndPoint`)) (`SceneComponent.K2_GetComponentLocation` (`self.StartPoint`))) (- (`self.Sum`) 1))))

(event `self.ReceiveTick`
  (params (DeltaSeconds :type "Float (single-precision)"))
  ;[1 1 1] Создаем предметы
  (bind _asglobal_variables (cast `/Game/Workplace/Blueprints/GlobalVariables` (`GameplayStatics.GetGameInstance`)))
  (if (>= (`/Game/Workplace/Blueprints/GlobalVariables.LevelPhase` _asglobal_variables) 4)
    (if (not (`self.LevelPhaseIsBiggerThan4`))
      (set `self.LevelPhaseIsBiggerThan4` true)
      (`self.CreateArm`)
      (`self.CreateArm`)
      (`self.CreateDirection`)
      (`self.CreateDirection`)
      (`self.CreateLidar`)
      (`self.CreateMotor`)
      (`self.CreateMotor`))))

(fn `Counter`
  (bind _asglobal_variables (cast `/Game/Workplace/Blueprints/GlobalVariables` (`GameplayStatics.GetGameInstance`)))
  (for (_array_element _array_index) (`/Game/Workplace/Blueprints/GlobalVariables.SDBoxGivenNum` _asglobal_variables)
    (bind _asglobal_variables_2 (cast `/Game/Workplace/Blueprints/GlobalVariables` (`GameplayStatics.GetGameInstance`)))
    (if (not (`|GetArrayItem` (`/Game/Workplace/Blueprints/GlobalVariables.SDPrintedObjects` _asglobal_variables_2) _array_index))
      (set `self.Sum` (+ (`self.Sum`) _array_element)))))

(fn `CreateArm`
  (bind _asglobal_variables (cast `/Game/Workplace/Blueprints/GlobalVariables` (`GameplayStatics.GetGameInstance`)))
  (bind _position (`self.GetPoint`))
  (bind _returnvalue (`|SpawnActorFromClass` "/Game/Workplace/Blueprints/BP_Shelf_Objects.BP_Shelf_Objects_C" (`KismetMathLibrary.MakeTransform` _position (`KismetMathLibrary.Conv_VectorToRotator` (`|GetArrayItem` (`/Game/Workplace/Blueprints/GlobalVariables.SDObjectsRotation` _asglobal_variables))) (`KismetMathLibrary.Conv_DoubleToVector` (`|GetArrayItem` (`/Game/Workplace/Blueprints/GlobalVariables.SDObjectsScale` _asglobal_variables)))) "Undefined" "OverrideRootScale" null null))
  (set `/Game/Workplace/Blueprints/BP_Shelf_Objects.SDIndex` 0 _returnvalue)
  (set `/Game/Workplace/Blueprints/BP_Shelf_Objects.Printed` false _returnvalue)
  (bind _asglobal_variables_2 (cast `/Game/Workplace/Blueprints/GlobalVariables` (`GameplayStatics.GetGameInstance`)))
  (bind _shelfobject (`/Game/Workplace/Blueprints/BP_Shelf_Objects.ShelfObject` _returnvalue))
  (`StaticMeshComponent.SetStaticMesh` _shelfobject (`|GetArrayItem` (`/Game/Workplace/Blueprints/GlobalVariables.SDObjects` _asglobal_variables_2)))
  (`PrimitiveComponent.SetSimulatePhysics` _shelfobject true)
  (`PrimitiveComponent.SetCollisionObjectType` _shelfobject "ECC_PhysicsBody"))

(fn `CreateDirection`
  (bind _asglobal_variables (cast `/Game/Workplace/Blueprints/GlobalVariables` (`GameplayStatics.GetGameInstance`)))
  (bind _position (`self.GetPoint`))
  (bind _returnvalue (`|SpawnActorFromClass` "/Game/Workplace/Blueprints/BP_Shelf_Objects.BP_Shelf_Objects_C" (`KismetMathLibrary.MakeTransform` _position (`KismetMathLibrary.Conv_VectorToRotator` (`|GetArrayItem` (`/Game/Workplace/Blueprints/GlobalVariables.SDObjectsRotation` _asglobal_variables) 1)) (`KismetMathLibrary.Conv_DoubleToVector` (`|GetArrayItem` (`/Game/Workplace/Blueprints/GlobalVariables.SDObjectsScale` _asglobal_variables) 1))) "Undefined" "OverrideRootScale" null null))
  (set `/Game/Workplace/Blueprints/BP_Shelf_Objects.SDIndex` 1 _returnvalue)
  (set `/Game/Workplace/Blueprints/BP_Shelf_Objects.Printed` false _returnvalue)
  (bind _asglobal_variables_2 (cast `/Game/Workplace/Blueprints/GlobalVariables` (`GameplayStatics.GetGameInstance`)))
  (bind _shelfobject (`/Game/Workplace/Blueprints/BP_Shelf_Objects.ShelfObject` _returnvalue))
  (`StaticMeshComponent.SetStaticMesh` _shelfobject (`|GetArrayItem` (`/Game/Workplace/Blueprints/GlobalVariables.SDObjects` _asglobal_variables_2) 1))
  (`PrimitiveComponent.SetSimulatePhysics` _shelfobject true)
  (`PrimitiveComponent.SetCollisionObjectType` _shelfobject "ECC_PhysicsBody"))

(fn `CreateLidar`
  (bind _asglobal_variables (cast `/Game/Workplace/Blueprints/GlobalVariables` (`GameplayStatics.GetGameInstance`)))
  (bind _position (`self.GetPoint`))
  (bind _returnvalue (`|SpawnActorFromClass` "/Game/Workplace/Blueprints/BP_Shelf_Objects.BP_Shelf_Objects_C" (`KismetMathLibrary.MakeTransform` _position (`KismetMathLibrary.Conv_VectorToRotator` (`|GetArrayItem` (`/Game/Workplace/Blueprints/GlobalVariables.SDObjectsRotation` _asglobal_variables) 5)) (`KismetMathLibrary.Conv_DoubleToVector` (`|GetArrayItem` (`/Game/Workplace/Blueprints/GlobalVariables.SDObjectsScale` _asglobal_variables) 5))) "Undefined" "OverrideRootScale" null null))
  (set `/Game/Workplace/Blueprints/BP_Shelf_Objects.SDIndex` 5 _returnvalue)
  (set `/Game/Workplace/Blueprints/BP_Shelf_Objects.Printed` false _returnvalue)
  (bind _asglobal_variables_2 (cast `/Game/Workplace/Blueprints/GlobalVariables` (`GameplayStatics.GetGameInstance`)))
  (bind _shelfobject (`/Game/Workplace/Blueprints/BP_Shelf_Objects.ShelfObject` _returnvalue))
  (`StaticMeshComponent.SetStaticMesh` _shelfobject (`|GetArrayItem` (`/Game/Workplace/Blueprints/GlobalVariables.SDObjects` _asglobal_variables_2) 5))
  (`PrimitiveComponent.SetSimulatePhysics` _shelfobject true)
  (`PrimitiveComponent.SetCollisionObjectType` _shelfobject "ECC_PhysicsBody"))

(fn `CreateMotor`
  (bind _asglobal_variables (cast `/Game/Workplace/Blueprints/GlobalVariables` (`GameplayStatics.GetGameInstance`)))
  (bind _position (`self.GetPoint`))
  (bind _returnvalue (`|SpawnActorFromClass` "/Game/Workplace/Blueprints/BP_Shelf_Objects.BP_Shelf_Objects_C" (`KismetMathLibrary.MakeTransform` _position (`KismetMathLibrary.Conv_VectorToRotator` (`|GetArrayItem` (`/Game/Workplace/Blueprints/GlobalVariables.SDObjectsRotation` _asglobal_variables) 7)) (`KismetMathLibrary.Conv_DoubleToVector` (`|GetArrayItem` (`/Game/Workplace/Blueprints/GlobalVariables.SDObjectsScale` _asglobal_variables) 7))) "Undefined" "OverrideRootScale" null null))
  (set `/Game/Workplace/Blueprints/BP_Shelf_Objects.SDIndex` 7 _returnvalue)
  (set `/Game/Workplace/Blueprints/BP_Shelf_Objects.Printed` false _returnvalue)
  (bind _asglobal_variables_2 (cast `/Game/Workplace/Blueprints/GlobalVariables` (`GameplayStatics.GetGameInstance`)))
  (bind _shelfobject (`/Game/Workplace/Blueprints/BP_Shelf_Objects.ShelfObject` _returnvalue))
  (`StaticMeshComponent.SetStaticMesh` _shelfobject (`|GetArrayItem` (`/Game/Workplace/Blueprints/GlobalVariables.SDObjects` _asglobal_variables_2) 7))
  (`PrimitiveComponent.SetSimulatePhysics` _shelfobject true)
  (`PrimitiveComponent.SetCollisionObjectType` _shelfobject "ECC_PhysicsBody"))

(fn `GetPoint`
  (returns (Position :type "Vector Structure"))
  (bind _output_get (set `self.NumberOfObject` (+ (`self.NumberOfObject`) 1)))
  (return (+ (`SceneComponent.K2_GetComponentLocation` (`self.StartPoint`)) (* (`self.Step`) (- _output_get 1)))))

(fn `UserConstructionScript`)