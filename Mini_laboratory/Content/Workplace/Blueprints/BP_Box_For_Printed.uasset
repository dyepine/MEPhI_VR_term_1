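; BP_Box_For_Printed is a box that collects printed SD objects and shows a delivered/required counter on BoxText.
; On BeginPlay it totals the GlobalVariables game instance quotas for the object types flagged as printed.
; DropObjectinBox counts a drop only if that type is printed and under quota, then updates the counter.
; Accepted materials and indexes are saved to the game instance, and PrintedReady is set once the total is reached.
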(event `self.ReceiveBeginPlay`
  ;[1 1 1] Задаем начальныые параметры
  (set `self.SDIndex` 0)
  (set `self.Material` null)
  (bind _asglobal_variables (cast `/Game/Workplace/Blueprints/GlobalVariables` (`GameplayStatics.GetGameInstance`)))
  (bind _output_get (set `self.NumObjects` (`/Game/Workplace/Blueprints/GlobalVariables.NumSDObjects` _asglobal_variables)))
  (for _ (range 1 (+ _output_get 1))
    (`KismetArrayLibrary.Array_Add` (`self.ObjectsGivenNum`)))
  (for (_array_element _array_index) (`/Game/Workplace/Blueprints/GlobalVariables.SDBoxGivenNum` _asglobal_variables)
    (bind _asglobal_variables_2 (cast `/Game/Workplace/Blueprints/GlobalVariables` (`GameplayStatics.GetGameInstance`)))
    (if (`|GetArrayItem` (`/Game/Workplace/Blueprints/GlobalVariables.SDPrintedObjects` _asglobal_variables_2) _array_index)
      (set `self.Sum` (+ (`self.Sum`) _array_element))))
  (`TextRenderComponent.K2_SetText` (`self.BoxText`) (`KismetTextLibrary.Conv_StringToText` (`KismetStringLibrary.Concat_StrStr` "0/" (`KismetStringLibrary.Conv_IntToString` (`self.Sum`)))))
  (set `self.NumGivenObjects` 0))

(event `/Game/Workplace/Blueprints/BI_Drop_In_Printed_Box.DropObjectInBox`
  (params (Material :type "Material Object Reference") (SDIndex :type Integer))
  (bind _sdindex (`self.SDIndex`))
  (bind _output (`|GetArrayItem` (`self.ObjectsGivenNum`) _sdindex))
  ;[1 1 1] Добавление объекта
  (set `self.Material` Material)
  (set `self.SDIndex` SDIndex)
  (bind _asglobal_variables (cast `/Game/Workplace/Blueprints/GlobalVariables` (`GameplayStatics.GetGameInstance`)))
  (if (`|GetArrayItem` (`/Game/Workplace/Blueprints/GlobalVariables.SDPrintedObjects` _asglobal_variables) (`self.SDIndex`))
    (bind _asglobal_variables_2 (cast `/Game/Workplace/Blueprints/GlobalVariables` (`GameplayStatics.GetGameInstance`)))
    (if (< _output (`|GetArrayItem` (`/Game/Workplace/Blueprints/GlobalVariables.SDBoxGivenNum` _asglobal_variables_2) _sdindex))
      (`KismetArrayLibrary.Array_Set` (`self.ObjectsGivenNum`) (`self.SDIndex`) (+ _output 1))
      (bind _output_get (set `self.NumGivenObjects` (+ (`self.NumGivenObjects`) 1)))
      (`TextRenderComponent.K2_SetText` (`self.BoxText`) (`KismetTextLibrary.Conv_StringToText` (`KismetStringLibrary.Concat_StrStr` (`KismetStringLibrary.Conv_IntToString` _output_get) "/" (`KismetStringLibrary.Conv_IntToString` (`self.Sum`)))))
      (if (> (`self.NumGivenObjects`) (`self.Sum`))
        (bind _asglobal_variables_3 (cast `/Game/Workplace/Blueprints/GlobalVariables` (`GameplayStatics.GetGameInstance`)))
        (set `/Game/Workplace/Blueprints/GlobalVariables.PrintedReady` true _asglobal_variables_3)
        (else
          (bind _asglobal_variables_4 (cast `/Game/Workplace/Blueprints/GlobalVariables` (`GameplayStatics.GetGameInstance`)))
          (`KismetArrayLibrary.Array_Add` (`/Game/Workplace/Blueprints/GlobalVariables.SDPRintedReadyMaterials` _asglobal_variables_4) (`self.Material`))
          (`KismetArrayLibrary.Array_Add` (`/Game/Workplace/Blueprints/GlobalVariables.SDPrintedReadyIndexes` _asglobal_variables_4) (`self.SDIndex`))
          (if (== (`self.NumGivenObjects`) (`self.Sum`))
            (bind _asglobal_variables_5 (cast `/Game/Workplace/Blueprints/GlobalVariables` (`GameplayStatics.GetGameInstance`)))
            (set `/Game/Workplace/Blueprints/GlobalVariables.PrintedReady` true _asglobal_variables_5)))))))

(fn `UserConstructionScript`)