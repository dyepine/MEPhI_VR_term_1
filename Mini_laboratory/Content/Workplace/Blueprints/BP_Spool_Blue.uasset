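; Blue spool actor whose parts (two frames and a plastic piece) change collision object type with level progress.
; Every Tick, it reads LevelPhase from the GlobalVariables game instance.
; From phase three onward all three components become PhysicsBody; before that they are WorldStatic.
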(event `self.ReceiveTick`
  (params (DeltaSeconds :type "Float (single-precision)"))
  (bind _asglobal_variables (cast `/Game/Workplace/Blueprints/GlobalVariables` (`GameplayStatics.GetGameInstance`)))
  (if (>= (`/Game/Workplace/Blueprints/GlobalVariables.LevelPhase` _asglobal_variables) 3)
    (`PrimitiveComponent.SetCollisionObjectType` (`self.Frame1`) "ECC_PhysicsBody")
    (`PrimitiveComponent.SetCollisionObjectType` (`self.Plastic`) "ECC_PhysicsBody")
    (`PrimitiveComponent.SetCollisionObjectType` (`self.Frame2`) "ECC_PhysicsBody")
    (else
      (`PrimitiveComponent.SetCollisionObjectType` (`self.Frame1`) "ECC_WorldStatic")
      (`PrimitiveComponent.SetCollisionObjectType` (`self.Plastic`) "ECC_WorldStatic")
      (`PrimitiveComponent.SetCollisionObjectType` (`self.Frame2`) "ECC_WorldStatic"))))

(fn `UserConstructionScript`)