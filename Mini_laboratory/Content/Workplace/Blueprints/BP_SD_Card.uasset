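; BP_SD_Card is a pickup actor for an SD card the player clicks to collect.
; Each Tick it reads the GlobalVariables game instance and checks whether it is the current HitResult while the left mouse button is pressed.
; From level phase three onward, such a click sets SDAvailable on the game instance and destroys the actor.
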(event `self.ReceiveTick`
  (params (DeltaSeconds :type "Float (single-precision)"))
  (bind _asglobal_variables (cast `/Game/Workplace/Blueprints/GlobalVariables` (`GameplayStatics.GetGameInstance`)))
  (if (== self (`/Game/Workplace/Blueprints/GlobalVariables.HitResult` _asglobal_variables))
    (if (`/Game/Workplace/Blueprints/GlobalVariables.LeftMousePressed` _asglobal_variables)
      (if (>= (`/Game/Workplace/Blueprints/GlobalVariables.LevelPhase` _asglobal_variables) 3)
        (set `/Game/Workplace/Blueprints/GlobalVariables.SDAvailable` true _asglobal_variables)
        (`self.K2_DestroyActor`)))))

(fn `UserConstructionScript`)