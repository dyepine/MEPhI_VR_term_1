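; BP_TableForDetails is a workplace table that lays out track objects in three rows of slots.
; BeginPlay fills LinePositions from each row's start marker, using the first row's step for all rows, leaving Step2 and Step3 unused.
; During level phase 1, AddObjectsonTable spawns a BP_ObjectOnTable at the indexed slot, with mesh and scale from GlobalVariables.
; It registers each object there and advances to phase 2 when ready and total track-object counts match.
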(event `self.ReceiveBeginPlay`
  (set `self.Step1` (/ (- (`SceneComponent.K2_GetComponentLocation` (`self.EndPosition1`)) (`SceneComponent.K2_GetComponentLocation` (`self.FirstPosition1`))) (- (`self.NumObjectsInLine`) 1)))
  (set `self.Step2` (/ (- (`SceneComponent.K2_GetComponentLocation` (`self.EndPosition2`)) (`SceneComponent.K2_GetComponentLocation` (`self.FirstPosition2`))) (- (`self.NumObjectsInLine`) 1)))
  (set `self.Step3` (/ (- (`SceneComponent.K2_GetComponentLocation` (`self.EndPosition3`)) (`SceneComponent.K2_GetComponentLocation` (`self.FirstPosition3`))) (- (`self.NumObjectsInLine`) 1)))
  (for _index (range (`self.NumObjectsInLine`))
    (`KismetArrayLibrary.Array_Add` (`self.LinePositions`) (+ (* (`self.Step1`) _index) (`SceneComponent.K2_GetComponentLocation` (`self.FirstPosition1`)))))
  (for _index_2 (range (`self.NumObjectsInLine`))
    (`KismetArrayLibrary.Array_Add` (`self.LinePositions`) (+ (* (`self.Step1`) _index_2) (`SceneComponent.K2_GetComponentLocation` (`self.FirstPosition2`)))))
  (for _index_3 (range (`self.NumObjectsInLine`))
    (`KismetArrayLibrary.Array_Add` (`self.LinePositions`) (+ (* (`self.Step1`) _index_3) (`SceneComponent.K2_GetComponentLocation` (`self.FirstPosition3`))))))

(event `/Game/Workplace/Blueprints/BI_AddObjectsOnTable.AddObjectsOnTable`
  (params (NumObject :type Integer))
  (bind _asglobal_variables (cast `/Game/Workplace/Blueprints/GlobalVariables` (`GameplayStatics.GetGameInstance`)))
  (if (== (`/Game/Workplace/Blueprints/GlobalVariables.LevelPhase` _asglobal_variables) 1)
    (bind _returnvalue (`|SpawnActorFromClass` "/Game/Workplace/Blueprints/BP_ObjectOnTable.BP_ObjectOnTable_C" (`KismetMathLibrary.MakeTransform` (`|GetArrayItem` (`self.LinePositions`) NumObject) (struct) (`KismetMathLibrary.Conv_DoubleToVector` (`|GetArrayItem` (`/Game/Workplace/Blueprints/GlobalVariables.ScaleObjectsOnTable` _asglobal_variables) NumObject))) "Undefined" "OverrideRootScale" null null))
    (bind _asglobal_variables_2 (cast `/Game/Workplace/Blueprints/GlobalVariables` (`GameplayStatics.GetGameInstance`)))
    (`StaticMeshComponent.SetStaticMesh` (`/Game/Workplace/Blueprints/BP_ObjectOnTable.ObjectOnTable` _returnvalue) (`|GetArrayItem` (`/Game/Workplace/Blueprints/GlobalVariables.ResultTrackObjects` _asglobal_variables_2) NumObject))
    (bind _asglobal_variables_3 (cast `/Game/Workplace/Blueprints/GlobalVariables` (`GameplayStatics.GetGameInstance`)))
    (`KismetArrayLibrary.Array_Add` (`/Game/Workplace/Blueprints/GlobalVariables.ObjectsOnTable` _asglobal_variables_3) _returnvalue)
    (if (== (`/Game/Workplace/Blueprints/GlobalVariables.NumTrackObjects` _asglobal_variables_3) (`/Game/Workplace/Blueprints/GlobalVariables.NumReadyTrackObjects` _asglobal_variables_3))
      (set `/Game/Workplace/Blueprints/GlobalVariables.LevelPhase` 2 _asglobal_variables_3))))

(fn `UserConstructionScript`)