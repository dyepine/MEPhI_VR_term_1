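; Workplace stamping machine that turns track objects into their finished versions and passes them on to the table.
; In level phase 1, AddObjectsonMachine spawns the indexed object on the machine using GameInstance mesh and scale arrays.
; Tick polls the GameInstance hit result for buttons by display name, gated by Edit/Send flags.
; After a delay, Edit swaps in the result mesh; Send destroys it, increments the ready count and notifies BI_AddObjectsOnTable actors.
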(event `self.ReceiveBeginPlay`
  (set `self.Edit` false)
  (set `self.Send` false))

(event `/Game/Workplace/Blueprints/BI_AddObjectsOnMachine.AddObjectsOnMachine`
  (params (NumObject :type Integer))
  (bind _asglobal_variables (cast `/Game/Workplace/Blueprints/GlobalVariables` (`GameplayStatics.GetGameInstance`)))
  (if (== (`/Game/Workplace/Blueprints/GlobalVariables.LevelPhase` _asglobal_variables) 1)
    (set `self.ObjectNumber` NumObject)
    (bind _asglobal_variables_2 (cast `/Game/Workplace/Blueprints/GlobalVariables` (`GameplayStatics.GetGameInstance`)))
    (if (< (`self.ObjectNumber`) (`/Game/Workplace/Blueprints/GlobalVariables.NumTrackObjects` _asglobal_variables_2))
      (bind _returnvalue (`|SpawnActorFromClass` "/Game/Workplace/Blueprints/BP_ObjectOnMachine.BP_ObjectOnMachine_C" (`KismetMathLibrary.MakeTransform` (`SceneComponent.K2_GetComponentLocation` (`self.PlaceForObject`)) (struct) (`KismetMathLibrary.Conv_DoubleToVector` (`|GetArrayItem` (`/Game/Workplace/Blueprints/GlobalVariables.ScaleTrackObjects` _asglobal_variables_2) (`self.ObjectNumber`)))) "Undefined" "OverrideRootScale" null null))
      (set `self.Object` _returnvalue)
      (bind _asglobal_variables_3 (cast `/Game/Workplace/Blueprints/GlobalVariables` (`GameplayStatics.GetGameInstance`)))
      (`StaticMeshComponent.SetStaticMesh` (`/Game/Workplace/Blueprints/BP_ObjectOnMachine.Object` _returnvalue) (`|GetArrayItem` (`/Game/Workplace/Blueprints/GlobalVariables.TrackObjects` _asglobal_variables_3) (`self.ObjectNumber`)))
      (set `self.Edit` true))))

(event `self.ReceiveTick`
  (params (DeltaSeconds :type "Float (single-precision)"))
  (`|ExecutionSequence`
    (:`then_0`
      (bind _asglobal_variables (cast `/Game/Workplace/Blueprints/GlobalVariables` (`GameplayStatics.GetGameInstance`)))
      (bind _asbp_button (cast `/Game/Workplace/Blueprints/BP_Button` (`/Game/Workplace/Blueprints/GlobalVariables.HitResult` _asglobal_variables)))
      (if (`KismetStringLibrary.EqualEqual_StrStr` (`KismetSystemLibrary.GetDisplayName` _asbp_button) "Edit_Button")
        (set `self.EditButton` _asbp_button)
        (if (`self.Edit`)
          (if (`KismetStringLibrary.EqualEqual_StrStr` (`KismetSystemLibrary.GetDisplayName` (`self.EditButton`)) "Edit_Button")
            (bind _asbp_button_2 (cast `/Game/Workplace/Blueprints/BP_Button` (`self.EditButton`)))
            (if (`/Game/Workplace/Blueprints/BP_Button.PreState` _asbp_button_2)
              (if (`/Game/Workplace/Blueprints/BP_Button.State` _asbp_button_2)
                (`KismetSystemLibrary.Delay` (`self.delay`))
                (bind _asbp_button_3 (cast `/Game/Workplace/Blueprints/BP_Button` (`self.EditButton`)))
                (set `/Game/Workplace/Blueprints/BP_Button.PreState` false _asbp_button_3)
                (set `/Game/Workplace/Blueprints/BP_Button.State` false _asbp_button_3)
                (set `self.Edit` false)
                (bind _asbp_object_on_machine (cast `/Game/Workplace/Blueprints/BP_ObjectOnMachine` (`self.Object`)))
                (bind _asglobal_variables_2 (cast `/Game/Workplace/Blueprints/GlobalVariables` (`GameplayStatics.GetGameInstance`)))
                (`StaticMeshComponent.SetStaticMesh` (`/Game/Workplace/Blueprints/BP_ObjectOnMachine.Object` _asbp_object_on_machine) (`|GetArrayItem` (`/Game/Workplace/Blueprints/GlobalVariables.ResultTrackObjects` _asglobal_variables_2) (`self.ObjectNumber`)))
                (set `self.Send` true)
                (bind _asbp_button_4 (cast `/Game/Workplace/Blueprints/BP_Button` (`self.EditButton`)))
                (set `/Game/Workplace/Blueprints/BP_Button.PreState` false _asbp_button_4)
                (set `/Game/Workplace/Blueprints/BP_Button.State` false _asbp_button_4))))
          (else
            (bind _asbp_button_5 (cast `/Game/Workplace/Blueprints/BP_Button` (`self.EditButton`)))
            (set `/Game/Workplace/Blueprints/BP_Button.PreState` false _asbp_button_5)
            (set `/Game/Workplace/Blueprints/BP_Button.State` false _asbp_button_5)))))
    (:`then_1`
      (bind _asglobal_variables_3 (cast `/Game/Workplace/Blueprints/GlobalVariables` (`GameplayStatics.GetGameInstance`)))
      (bind _asbp_button_6 (cast `/Game/Workplace/Blueprints/BP_Button` (`/Game/Workplace/Blueprints/GlobalVariables.HitResult` _asglobal_variables_3)))
      (if (`KismetStringLibrary.EqualEqual_StrStr` (`KismetSystemLibrary.GetDisplayName` _asbp_button_6) "Send_Button")
        (set `self.SendButton` _asbp_button_6)
        (if (`self.Send`)
          (if (`KismetStringLibrary.EqualEqual_StrStr` (`KismetSystemLibrary.GetDisplayName` (`self.SendButton`)) "Send_Button")
            (bind _asbp_button_7 (cast `/Game/Workplace/Blueprints/BP_Button` (`self.SendButton`)))
            (if (`/Game/Workplace/Blueprints/BP_Button.PreState` _asbp_button_7)
              (if (`/Game/Workplace/Blueprints/BP_Button.State` _asbp_button_7)
                (`KismetSystemLibrary.Delay` (`self.delay`))
                (bind _asbp_button_8 (cast `/Game/Workplace/Blueprints/BP_Button` (`self.SendButton`)))
                (set `/Game/Workplace/Blueprints/BP_Button.PreState` false _asbp_button_8)
                (set `/Game/Workplace/Blueprints/BP_Button.State` false _asbp_button_8)
                (set `self.Send` false)
                (`self.K2_DestroyActor` (`self.Object`))
                (bind _outactors (`GameplayStatics.GetAllActorsWithInterface` "/Game/Workplace/Blueprints/BI_AddObjectsOnTable.BI_AddObjectsOnTable_C"))
                (bind _asglobal_variables_4 (cast `/Game/Workplace/Blueprints/GlobalVariables` (`GameplayStatics.GetGameInstance`)))
                (set `/Game/Workplace/Blueprints/GlobalVariables.NumReadyTrackObjects` (+ (`/Game/Workplace/Blueprints/GlobalVariables.NumReadyTrackObjects` _asglobal_variables_4) 1) _asglobal_variables_4)
                (message `/Game/Workplace/Blueprints/BI_AddObjectsOnTable.AddObjectsOnTable` _outactors (`self.ObjectNumber`))
                (bind _asbp_button_9 (cast `/Game/Workplace/Blueprints/BP_Button` (`self.SendButton`)))
                (set `/Game/Workplace/Blueprints/BP_Button.PreState` false _asbp_button_9)
                (set `/Game/Workplace/Blueprints/BP_Button.State` false _asbp_button_9))))
          (else
            (bind _asbp_button_10 (cast `/Game/Workplace/Blueprints/BP_Button` (`self.SendButton`)))
            (set `/Game/Workplace/Blueprints/BP_Button.PreState` false _asbp_button_10)
            (set `/Game/Workplace/Blueprints/BP_Button.State` false _asbp_button_10)))))))

(fn `UserConstructionScript`)