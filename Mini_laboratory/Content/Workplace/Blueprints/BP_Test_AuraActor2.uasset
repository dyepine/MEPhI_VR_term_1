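; BP_Test_AuraActor2 is a test actor that shows its BlueCube component as a highlight when it is the current hit target.
; Each Tick, it casts the game instance to GlobalVariables and reads the shared Visible flag and HitResult.
; The cube is visible only while Visible is true and HitResult is this actor, and is hidden otherwise.
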(event `self.ReceiveTick`
  (params (DeltaSeconds :type "Float (single-precision)"))
  (bind _asglobal_variables (cast `/Game/Workplace/Blueprints/GlobalVariables` (`GameplayStatics.GetGameInstance`)))
  (if (`/Game/Workplace/Blueprints/GlobalVariables.Visible` _asglobal_variables)
    (if (== self (`/Game/Workplace/Blueprints/GlobalVariables.HitResult` _asglobal_variables))
      (`SceneComponent.SetVisibility` (`self.Blue_cube`) true true)
      (else
        (`SceneComponent.SetVisibility` (`self.Blue_cube`) false false)))
    (else
      (`SceneComponent.SetVisibility` (`self.Blue_cube`) false false))))

(fn `UserConstructionScript`)