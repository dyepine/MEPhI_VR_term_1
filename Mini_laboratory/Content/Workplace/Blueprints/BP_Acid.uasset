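; BP_Acid is an acid station that changes the plastic of printed shelf objects to an acided variant.
; On collision overlap, it matches an un-acided BP_Shelf_Objects' blue, red, green or yellow material, swaps it and sets the Acided flag.
; Each Tick, it reads mouse state and hit object from GlobalVariables, showing its Aura while left mouse is pressed on a printed, un-acided shelf object.
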(event `self.Collision.OnComponentBeginOverlap`
  (params (OverlappedComponent :type "PrimitiveComponent Object Reference") (OtherActor :type "Actor Object Reference") (OtherComp :type "PrimitiveComponent Object Reference") (OtherBodyIndex :type Integer) (bFromSweep :type Boolean) (SweepResult :type "HitResult Structure (by ref)"))
  ;[1 1 1] Меняем цвет пластика
  (bind _asbp_shelf_objects (cast `/Game/Workplace/Blueprints/BP_Shelf_Objects` OtherActor))
  (if (`/Game/Workplace/Blueprints/BP_Shelf_Objects.Printed` _asbp_shelf_objects)
    (if (not (`/Game/Workplace/Blueprints/BP_Shelf_Objects.Acided` _asbp_shelf_objects))
      (`|ExecutionSequence`
        (:`then_0`
          (bind _material (`/Game/Workplace/Blueprints/BP_Shelf_Objects.Material` _asbp_shelf_objects))
          (if (== _material "/Game/Workplace/Materials/M_Plastic_Blue.M_Plastic_Blue")
            (set `/Game/Workplace/Blueprints/BP_Shelf_Objects.Acided` true _asbp_shelf_objects)
            (set `/Game/Workplace/Blueprints/BP_Shelf_Objects.Material` "/Game/Workplace/Materials/M_Plastic_Blue_Acided.M_Plastic_Blue_Acided" _asbp_shelf_objects)
            (bind _shelfobject (`/Game/Workplace/Blueprints/BP_Shelf_Objects.ShelfObject` _asbp_shelf_objects))
            (`PrimitiveComponent.SetMaterial` _shelfobject 0 "/Game/Workplace/Materials/M_Plastic_Blue_Acided.M_Plastic_Blue_Acided")))
        (:`then_1`
          (if (== _material "/Game/Workplace/Materials/M_Plastic_Red.M_Plastic_Red")
            (set `/Game/Workplace/Blueprints/BP_Shelf_Objects.Acided` true _asbp_shelf_objects)
            (set `/Game/Workplace/Blueprints/BP_Shelf_Objects.Material` "/Game/Workplace/Materials/M_Plastic_Red_Acided.M_Plastic_Red_Acided" _asbp_shelf_objects)
            (`PrimitiveComponent.SetMaterial` _shelfobject 0 "/Game/Workplace/Materials/M_Plastic_Red_Acided.M_Plastic_Red_Acided")))
        (:`then_2`
          (if (== _material "/Game/Workplace/Materials/M_Plastic_Green.M_Plastic_Green")
            (set `/Game/Workplace/Blueprints/BP_Shelf_Objects.Acided` true _asbp_shelf_objects)
            (set `/Game/Workplace/Blueprints/BP_Shelf_Objects.Material` "/Game/Workplace/Materials/M_Plastic_Green_Acided.M_Plastic_Green_Acided" _asbp_shelf_objects)
            (`PrimitiveComponent.SetMaterial` _shelfobject 0 "/Game/Workplace/Materials/M_Plastic_Green_Acided.M_Plastic_Green_Acided")))
        (:`then_3`
          (if (== _material "/Game/Workplace/Materials/M_Plastic_Yellow.M_Plastic_Yellow")
            (set `/Game/Workplace/Blueprints/BP_Shelf_Objects.Acided` true _asbp_shelf_objects)
            (set `/Game/Workplace/Blueprints/BP_Shelf_Objects.Material` "/Game/Workplace/Materials/M_Plastic_Yellow_Acided.M_Plastic_Yellow_Acided" _asbp_shelf_objects)
            (`PrimitiveComponent.SetMaterial` _shelfobject 0 "/Game/Workplace/Materials/M_Plastic_Yellow_Acided.M_Plastic_Yellow_Acided")))))))

(event `self.ReceiveTick`
  (params (DeltaSeconds :type "Float (single-precision)"))
  ;[1 1 1] Добавляем ауру
  (bind _asglobal_variables (cast `/Game/Workplace/Blueprints/GlobalVariables` (`GameplayStatics.GetGameInstance`)))
  (if (`/Game/Workplace/Blueprints/GlobalVariables.LeftMousePressed` _asglobal_variables)
    (bind _asbp_shelf_objects (cast `/Game/Workplace/Blueprints/BP_Shelf_Objects` (`/Game/Workplace/Blueprints/GlobalVariables.HitResult` _asglobal_variables)))
    (if (`/Game/Workplace/Blueprints/BP_Shelf_Objects.Printed` _asbp_shelf_objects)
      (if (`/Game/Workplace/Blueprints/BP_Shelf_Objects.Acided` _asbp_shelf_objects)
        (`SceneComponent.SetVisibility` (`self.Aura`) false false)
        (else
          (`SceneComponent.SetVisibility` (`self.Aura`) true false)))
      (else
        (`SceneComponent.SetVisibility` (`self.Aura`) false false)))
    (else
      (`SceneComponent.SetVisibility` (`self.Aura`) false false))))

(fn `UserConstructionScript`)