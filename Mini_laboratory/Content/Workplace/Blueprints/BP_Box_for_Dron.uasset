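; BP_Box_for_Dron is a drop box that collects required non-printed objects and shows progress on BoxText.
; On BeginPlay it reads the GlobalVariables game instance, totals the quotas of non-printed object types and zeroes per-type counters.
; A BP_GivenObjects actor overlapping Collision is counted and destroyed if its type is non-printed and under quota.
; Reaching the total sets UnprintedReady on the game instance.
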(event `self.Collision.OnComponentBeginOverlap`
  (params (OverlappedComponent :type "PrimitiveComponent Object Reference") (OtherActor :type "Actor Object Reference") (OtherComp :type "PrimitiveComponent Object Reference") (OtherBodyIndex :type Integer) (bFromSweep :type Boolean) (SweepResult :type "HitResult Structure (by ref)"))
  ;[1 1 1] Добавление объекта
  (bind _asbp_given_objects (cast `/Game/Workplace/Blueprints/BP_GivenObjects` OtherActor))
  (bind _asglobal_variables (cast `/Game/Workplace/Blueprints/GlobalVariables` (`GameplayStatics.GetGameInstance`)))
  (bind _index (`/Game/Workplace/Blueprints/BP_GivenObjects.Index` _asbp_given_objects))
  (if (not (`|GetArrayItem` (`/Game/Workplace/Blueprints/GlobalVariables.SDPrintedObjects` _asglobal_variables) _index))
    (bind _asglobal_variables_2 (cast `/Game/Workplace/Blueprints/GlobalVariables` (`GameplayStatics.GetGameInstance`)))
    (bind _output (`|GetArrayItem` (`self.ObjectsGivenNum`) _index))
    (if (< _output (`|GetArrayItem` (`/Game/Workplace/Blueprints/GlobalVariables.SDBoxGivenNum` _asglobal_variables_2) _index))
      (`KismetArrayLibrary.Array_Set` (`self.ObjectsGivenNum`) _index (+ _output 1))
      (bind _output_get (set `self.NumGivenObjects` (+ (`self.NumGivenObjects`) 1)))
      (`TextRenderComponent.K2_SetText` (`self.BoxText`) (`KismetTextLibrary.Conv_StringToText` (`KismetStringLibrary.Concat_StrStr` (`KismetStringLibrary.Conv_IntToString` _output_get) "/" (`KismetStringLibrary.Conv_IntToString` (`self.Sum`)))))
      (`self.K2_DestroyActor` OtherActor)
      (if (>= (`self.NumGivenObjects`) (`self.Sum`))
        (bind _asglobal_variables_3 (cast `/Game/Workplace/Blueprints/GlobalVariables` (`GameplayStatics.GetGameInstance`)))
        (set `/Game/Workplace/Blueprints/GlobalVariables.UnprintedReady` true _asglobal_variables_3)))))

(event `self.ReceiveBeginPlay`
  ;[1 1 1] Задаем начальныые параметры
  (bind _asglobal_variables (cast `/Game/Workplace/Blueprints/GlobalVariables` (`GameplayStatics.GetGameInstance`)))
  (bind _output_get (set `self.NumObjects` (`/Game/Workplace/Blueprints/GlobalVariables.NumSDObjects` _asglobal_variables)))
  (for _ (range 1 (+ _output_get 1))
    (`KismetArrayLibrary.Array_Add` (`self.ObjectsGivenNum`)))
  (for (_array_element _array_index) (`/Game/Workplace/Blueprints/GlobalVariables.SDBoxGivenNum` _asglobal_variables)
    (bind _asglobal_variables_2 (cast `/Game/Workplace/Blueprints/GlobalVariables` (`GameplayStatics.GetGameInstance`)))
    (if (not (`|GetArrayItem` (`/Game/Workplace/Blueprints/GlobalVariables.SDPrintedObjects` _asglobal_variables_2) _array_index))
      (set `self.Sum` (+ (`self.Sum`) _array_element))))
  (`TextRenderComponent.K2_SetText` (`self.BoxText`) (`KismetTextLibrary.Conv_StringToText` (`KismetStringLibrary.Concat_StrStr` "0/" (`KismetStringLibrary.Conv_IntToString` (`self.Sum`)))))
  (set `self.NumGivenObjects` 0))

(fn `UserConstructionScript`)